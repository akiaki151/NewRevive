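; Manager actor that controls how many MapGoEfectBP effect actors exist, based on the player character's PHP value.
; Each Tick it picks a cap from PHP thresholds, then spawns one effect at the world origin while its counter is within that cap.
; If either NotUpDown flag on the player is set, it destroys all effects and resets the counter.
; Below the lowest threshold it neither spawns nor clears.
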(event EventBeginPlay)

(event EventTick
  (params (DeltaSeconds :type Float%20%28single-precision%29))
  (bind _returnvalue (Game|Player|GetPlayerPawn 0))
  (bind _returnvalue_2 (Game|Player|GetPlayerPawn 0))
  (bind _asthird_person_character (Utilities|Casting|CastToThirdPersonCharacter _returnvalue))
  (bind _asthird_person_character_2 (Utilities|Casting|CastToThirdPersonCharacter _returnvalue_2))
  (bind _p_hp (Variables|/Game/Revive/Blueprints/Character/ThirdPersonCharacter.ThirdPersonCharacter_C|GetP_HP _asthird_person_character_2))
  (if (<= 6e+01 _p_hp)
    (Variables|Default|SetProportional_HP_MAX 60)
    (if (Variables|/Game/Revive/Blueprints/Character/ThirdPersonCharacter.ThirdPersonCharacter_C|GetNot%20Up%20Down _asthird_person_character) :!label _label
      (bind _outactors (Actor|GetAllActorsOfClass "/Game/Revive/Blueprints/Character/MapGoEfectBP.MapGoEfectBP_C" :!label _label_2))
      (Variables|Default|SetMaxFire 0)
      (for _array_element _outactors
        (Actor|DestroyActor _array_element))
      (elif (Variables|/Game/Revive/Blueprints/Character/ThirdPersonCharacter.ThirdPersonCharacter_C|GetNotUpDown2 _asthird_person_character)
        (goto _label_2)
        (elif (<= (Variables|Default|GetMaxFire) (Variables|Default|GetProportional_HP_MAX))
          (Game|SpawnActorfromClass "/Game/Revive/Blueprints/Character/MapGoEfectBP.MapGoEfectBP_C" (Math|Transform|MakeTransform "0, 0, 0") "Undefined" 0 0)
          (Variables|Default|SetMaxFire (+ (Variables|Default|GetMaxFire) 1)))))
    (elif (<= 3e+01 _p_hp)
      (Variables|Default|SetProportional_HP_MAX 6)
      (goto _label)
      (elif (<= 15.0 _p_hp)
        (Variables|Default|SetProportional_HP_MAX 1)
        (goto _label)))))

(fn ConstructionScript)