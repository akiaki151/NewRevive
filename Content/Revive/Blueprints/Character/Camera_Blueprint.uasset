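; Camera actor that follows the player pawn and serves as the player's view.
; On BeginPlay it becomes the view target of player controller 0 and limits the camera manager's view pitch to a symmetric range.
; Every Tick it snaps to the pawn's location and copies its control rotation, with no interpolation or sweep.
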(event EventBeginPlay
  (bind _returnvalue (Game|GetPlayerCameraManager 0))
  (Game|Player|SetViewTargetwithBlend (Game|GetPlayerController 0) self 0.0 "VTBlend_Linear" 0.0 false)
  (Variables|/Script/Engine.PlayerCameraManager|SetViewPitchMax _returnvalue 45.0)
  (Variables|/Script/Engine.PlayerCameraManager|SetViewPitchMin _returnvalue -45.0))

(event Collision|EventActorBeginOverlap
  (params (OtherActor :type Actor%20Object%20Reference)))

(event EventTick
  (params (DeltaSeconds :type Float%20%28single-precision%29))
  (bind _returnvalue (Game|Player|GetPlayerPawn 0))
  ;[1 1 1] プレイヤーにカメラが追従するように設定
  (Transformation|SetActorLocation (Transformation|GetActorLocation _returnvalue) false false)
  (Transformation|SetActorRotation (Pawn|GetControlRotation _returnvalue :!class /Script/Engine.Pawn)))

(fn ConstructionScript)