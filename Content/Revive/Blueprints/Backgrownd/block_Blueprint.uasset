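; Background block actor that builds a scattered field of mesh pieces and moves vertically during play.
; The construction script spawns a WidthCount by LengthCount grid of StaticMesh components at 100-unit spacing, each with random uniform scale and random orientation, which overrides the alternating initial tilt.
; On BeginPlay, UPMove selects one of two timelines whose track value drives a per-update Z offset, with opposite sign for each.
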(event EventBeginPlay
  (if (Variables|Default|GetUPMove?)
    (bind _新規track_0 (Timeline|タイムライン_0 Play)
      (:Update
        (Transformation|AddActorLocalOffset (Math|Vector|MakeVector 0.0 0.0 (* _新規track_0 0.5)) false false)))
    (else
      (bind _新規track_0_2 (Timeline|タイムライン_1 Play)
        (:Update
          (Transformation|AddActorLocalOffset (Math|Vector|MakeVector 0.0 0.0 (* _新規track_0_2 -0.5)) false false))))))

(fn ConstructionScript
  (for _index (range 1 (Variables|Default|GetWidthCount)) ; 横幅のカウント
    (for _index_2 (range 1 (Variables|Default|GetLengthCount)) ; 縦幅のカウント
      (if (<= (Math|Integer|%(Integer) (Variables|Default|Getfor_index) 2) 0)
        (Variables|Default|SetRotation "0, 0, 0")
        (else
          (Variables|Default|SetRotation "22.000000,22.000000,22.000000")))
      (bind _returnvalue (AddComponent|AddStaticMeshComponent false (Math|Transform|MakeTransform (Math|Vector|MakeVector (* (- _index 1) 1e+02) (* (- _index_2 1) 1e+02) 0.0) (Variables|Default|GetRotation))))
      (bind _output_get (Variables|Default|Setfor_index (+ (Variables|Default|Getfor_index) 1)))
      (Components|StaticMesh|SetStaticMesh _returnvalue (Variables|Default|GetStaticMesh))
      (Transformation|SetWorldScale3D _returnvalue (Math|Conversions|ToVector(Float) (Math|Random|RandomFloatinRange 0.0 1.0)))
      (Transformation|SetWorldRotation _returnvalue (Math|Conversions|RotationFromXVector (Math|Conversions|ToVector(Float) (Utilities|Struct|MakeIntVector (Math|Random|RandomIntegerinRange 1 360) (Math|Random|RandomIntegerinRange 1 360) (Math|Random|RandomIntegerinRange 1 360)))) false false))))