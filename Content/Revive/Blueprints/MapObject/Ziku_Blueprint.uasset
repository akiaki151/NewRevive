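; Ziku_Blueprint is a map object, apparently an axis ("ziku"), that notifies nearby Wakusei (planet) actors when they are inside its radius.
; The construction script sizes the sphere, scales the mesh and snaps the actor to an upper or lower height from UpdownJudge.
; Each Tick it scans all Wakusei actors on the same layer, tests squared XY distance instead of using overlaps, and sends ZikuHanniMessage with the offset vector.
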(event OnComponentBeginOverlap(Box)
  (params (OverlappedComponent :type Primitive%20Component%20Object%20Reference) (OtherActor :type Actor%20Object%20Reference) (OtherComp :type Primitive%20Component%20Object%20Reference) (OtherBodyIndex :type Integer) (bFromSweep :type Boolean) (SweepResult :type Hit%20Result%20Structure%20%28by%20ref%29)))

(event OnComponentEndOverlap(Box)
  (params (OverlappedComponent :type Primitive%20Component%20Object%20Reference) (OtherActor :type Actor%20Object%20Reference) (OtherComp :type Primitive%20Component%20Object%20Reference) (OtherBodyIndex :type Integer)))

(event EventBeginPlay
  (Components|Sphere|SetSphereRadius (Variables|Default|GetSphere) (Variables|Default|GetRadius) true))

(event Collision|EventActorBeginOverlap
  (params (OtherActor :type Actor%20Object%20Reference)))

(event EventTick
  (params (DeltaSeconds :type Float%20%28single-precision%29))
  (bind _staticmeshcomponent (Variables|Debug|GetStaticMeshComponent))
  (bind _returnvalue (Transformation|GetWorldLocation _staticmeshcomponent))
  (bind _outactors (Actor|GetAllActorsOfClass "/Game/Revive/Blueprints/MapObject/Wakusei_Blueprint.Wakusei_Blueprint_C"))
  (for _array_element _outactors
    (if (Math|Boolean|Equal(Boolean) (Variables|Default|GetUpdownJudge) (Variables|/Game/Revive/Blueprints/MapObject/Wakusei_Blueprint.Wakusei_Blueprint_C|GetUpdown_Judge _array_element))
      (if (< (+ (* (- (.x (Transformation|GetWorldLocation (Variables|/Script/Engine.StaticMeshActor|GetStaticMeshComponent _array_element))) (.x _returnvalue)) (- (.x (Transformation|GetWorldLocation (Variables|/Script/Engine.StaticMeshActor|GetStaticMeshComponent _array_element))) (.x _returnvalue))) (* (- (.y (Transformation|GetWorldLocation (Variables|/Script/Engine.StaticMeshActor|GetStaticMeshComponent _array_element))) (.y _returnvalue)) (- (.y (Transformation|GetWorldLocation (Variables|/Script/Engine.StaticMeshActor|GetStaticMeshComponent _array_element))) (.y _returnvalue)))) (* (Variables|Default|GetRadius) (Variables|Default|GetRadius)))
        (Class|ZikuHanniBPIF|ZikuHanni(Message) _array_element true (- (Transformation|GetWorldLocation (Variables|/Script/Engine.StaticMeshActor|GetStaticMeshComponent _array_element)) (Transformation|GetWorldLocation (Variables|Debug|GetStaticMeshComponent))))))))

(fn ConstructionScript
  (bind _returnvalue (Transformation|GetActorLocation))
  (Components|Sphere|SetSphereRadius (Variables|Default|GetSphere) (Variables|Default|GetRadius) true)
  (Transformation|SetWorldScale3D (Variables|Debug|GetStaticMeshComponent) "5.000000,5.000000,5.000000")
  (if (Variables|Default|GetUpdownJudge)
    (Variables|Default|SetZ_Location 1.16e+03)
    (else
      (Variables|Default|SetZ_Location 2.3e+02)))
  (Transformation|SetActorLocation (Math|Vector|MakeVector (.x _returnvalue) (.y _returnvalue) (Variables|Default|GetZ_Location)) false false))