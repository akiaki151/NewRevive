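; Child Blueprint for an ice planet (Wakusei) map object that shares its HP (PHP) with nearby planets.
; Each Tick scales blast, range and collision components by PHP, writing it to IceGetHp on overlapping regular and energy planets with matching UpdownJudge.
; A separate check zeroes that value when OtherActor stops overlapping.
; Tick also toggles ice particles by HP, shows the range cylinder by player side, and spawns the Suikomi widget on player line hits.
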(event OnComponentEndOverlap(Sphere)
  (params (OverlappedComponent :type Primitive%20Component%20Object%20Reference) (OtherActor :type Actor%20Object%20Reference) (OtherComp :type Primitive%20Component%20Object%20Reference) (OtherBodyIndex :type Integer))
  ;[1 1 1] COLLISION
)

(event EventBeginPlay
  ;[1 1 1] BEGIN
  (|CallParentFunction))

(event Collision|EventActorBeginOverlap
  (params (OtherActor :type Actor%20Object%20Reference))
  (|CallParentFunction OtherActor) ; This node is disabled and will not be called.\nDrag off pins to build functionality.
)

(event EventTick
  (params (DeltaSeconds :type Float%20%28single-precision%29))
  (bind _p_hp (Variables|Default|GetP_HP))
  (bind _p_hp_2 (Variables|Default|GetP_HP))
  (bind _cylinder (Variables|Default|GetCylinder))
  (bind _iceplanet (Variables|Default|Geticeplanet))
  (bind _returnvalue (* _p_hp_2 0.25))
  (bind _returnvalue_2 (* _p_hp 0.4))
  ;[1 1 1] UPDATE
  (|CallParentFunction DeltaSeconds)
  (Development|PrintString (Utilities|String|ToString(Boolean) (Variables|Default|GetIceFlag)) true true "(R=0.278120,G=1.000000,B=0.000000,A=1.000000)" 0.0)
  (Utilities|FlowControl|Sequence
    (:then_0
      (bind _output_get (Variables|Default|SetBakuhaHanni (Math|Conversions|ToVector(Float) (* (Variables|Default|GetP_HP) 0.5))))
      (Transformation|SetWorldScale3D (Variables|Default|Getbakuha) _output_get))
    (:then_1
      (if (Variables|Default|GetPlayer_In)
        (if (Variables|Default|Getplayer_hit)
          (if (>= (Variables|Default|GetP_HP) 0.0)
            (bind _asthird_person_character (Utilities|Casting|CastToThirdPersonCharacter (Game|GetPlayerCharacter 0)))
            (if (not (Variables|/Game/Revive/Blueprints/Character/ThirdPersonCharacter.ThirdPersonCharacter_C|GetNoInput _asthird_person_character))
              (if (Variables|/Game/Revive/Blueprints/Character/ThirdPersonCharacter.ThirdPersonCharacter_C|Getline_hit _asthird_person_character)
                (bind _returnvalue_3 (UserInterface|CreateWidget "/Game/Revive/Blueprints/UI/Suikomi_UI.Suikomi_UI_C"))
                (UserInterface|Viewport|AddtoViewport _returnvalue_3 0)))))))
    (:then_2
      (bind _outactors (Actor|GetAllActorsOfClass "/Game/Revive/Blueprints/MapObject/Wakusei_Blueprint.Wakusei_Blueprint_C"))
      (for _array_element _outactors
        (bind _aswakusei_blueprint (Utilities|Casting|CastToWakusei_Blueprint _array_element))
        (if (Class|PrimitiveComponent|IsOverlappingComponent (Variables|Default|GetIce_collision) (Variables|/Game/Revive/Blueprints/MapObject/Wakusei_Blueprint.Wakusei_Blueprint_C|GetSphere1 _aswakusei_blueprint))
          (if (Math|Boolean|Equal(Boolean) (Variables|Default|GetUpdown_Judge) (Variables|/Game/Revive/Blueprints/MapObject/Wakusei_Blueprint.Wakusei_Blueprint_C|GetUpdown_Judge _aswakusei_blueprint))
            (Variables|/Game/Revive/Blueprints/MapObject/Wakusei_Blueprint.Wakusei_Blueprint_C|SetIceGetHp _aswakusei_blueprint (Variables|Default|GetP_HP))))))
    (:then_3
      (bind _outactors_2 (Actor|GetAllActorsOfClass "/Game/Revive/Blueprints/MapObject/EnergieWakusei_Blueprint.EnergieWakusei_Blueprint_C"))
      (for _array_element_2 _outactors_2
        (bind _asenergie_wakusei_blueprint (Utilities|Casting|CastToEnergieWakusei_Blueprint _array_element_2))
        (if (Class|PrimitiveComponent|IsOverlappingComponent (Variables|Default|GetIce_collision) (Variables|/Game/Revive/Blueprints/MapObject/EnergieWakusei_Blueprint.EnergieWakusei_Blueprint_C|GetSphere1 _asenergie_wakusei_blueprint))
          (if (Math|Boolean|Equal(Boolean) (Variables|Default|GetUpdown_Judge) (Variables|/Game/Revive/Blueprints/MapObject/EnergieWakusei_Blueprint.EnergieWakusei_Blueprint_C|GetUpdown_Judge _asenergie_wakusei_blueprint))
            (Variables|/Game/Revive/Blueprints/MapObject/EnergieWakusei_Blueprint.EnergieWakusei_Blueprint_C|SetIceGetHp _asenergie_wakusei_blueprint (Variables|Default|GetP_HP))))))
    (:then_4
      ;[1 1 1] COLLISION
      (Utilities|FlowControl|Sequence
        (:then_0
          ;;[1 1 1] wakuseiがIceWakuseiと当たっていなかったらWakuseiの体力に０を代入する
          (if (Utilities|IsValid (stale OnComponentEndOverlap(Sphere) OtherActor))
            (if (Utilities|ClassIsChildOf (Utilities|GetClass (stale OnComponentEndOverlap(Sphere) OtherActor)) "/Game/Revive/Blueprints/MapObject/Wakusei_Blueprint.Wakusei_Blueprint_C")
              (bind _aswakusei_blueprint_2 (Utilities|Casting|CastToWakusei_Blueprint (stale OnComponentEndOverlap(Sphere) OtherActor)))
              (if (not (Class|PrimitiveComponent|IsOverlappingComponent (Variables|Default|GetIce_collision) (Variables|/Game/Revive/Blueprints/MapObject/Wakusei_Blueprint.Wakusei_Blueprint_C|GetSphere1 _aswakusei_blueprint_2)))
                (Variables|/Game/Revive/Blueprints/MapObject/Wakusei_Blueprint.Wakusei_Blueprint_C|SetIceGetHp _aswakusei_blueprint_2 0.0)))))
        (:then_1
          ;;[1 1 1] EnergiewakuseiがIceWakuseiと当たっていなかったらEnergieWakuseiの体力に０を代入する
          (if (Utilities|ClassIsChildOf (Utilities|GetClass (stale OnComponentEndOverlap(Sphere) OtherActor)) "/Game/Revive/Blueprints/MapObject/EnergieWakusei_Blueprint.EnergieWakusei_Blueprint_C")
            (bind _asenergie_wakusei_blueprint_2 (Utilities|Casting|CastToEnergieWakusei_Blueprint (stale OnComponentEndOverlap(Sphere) OtherActor)))
            (if (not (Class|PrimitiveComponent|IsOverlappingComponent (Variables|Default|GetIce_collision) (Variables|/Game/Revive/Blueprints/MapObject/EnergieWakusei_Blueprint.EnergieWakusei_Blueprint_C|GetSphere1 _asenergie_wakusei_blueprint_2)))
              (Variables|/Game/Revive/Blueprints/MapObject/EnergieWakusei_Blueprint.EnergieWakusei_Blueprint_C|SetIceGetHp _asenergie_wakusei_blueprint_2 0.0))))))
    (:then_5
      (Transformation|SetWorldScale3D (Variables|Default|GetPlayerhit) (Utilities|DEFINEWAKUSEILINEHITSCALE))
      (Transformation|SetWorldScale3D (Variables|Default|GetHP) "2.500000,2.500000,2.500000")
      (Transformation|SetWorldScale3D (Variables|Default|GetCylinder) (Math|Vector|MakeVector _returnvalue _returnvalue 0.0))
      (Transformation|SetWorldScale3D (Variables|Default|GetIce_collision) (Math|Vector|MakeVector _returnvalue_2 _returnvalue_2 _returnvalue_2)))
    (:then_6
      (if (> (Variables|Default|GetP_HP) 0.0)
        (Components|Activation|Activate _iceplanet false) ; パーティクル再生
        (else
          (Components|Activation|Deactivate _iceplanet) ; パーティクル停止
        )))
    (:then_7
      (bind _outactors_3 (Actor|GetAllActorsOfClass "/Game/Revive/Blueprints/Character/ThirdPersonCharacter.ThirdPersonCharacter_C"))
      (for _array_element_3 _outactors_3
        (if (Math|Boolean|Equal(Boolean) (Variables|Default|GetUpdown_Judge) (Variables|/Game/Revive/Blueprints/Character/ThirdPersonCharacter.ThirdPersonCharacter_C|GetPlayerUP _array_element_3))
          (Rendering|SetVisibility _cylinder true false)
          (else
            (Rendering|SetVisibility _cylinder false false)))))))

(fn ConstructionScript
  (bind _p_hp (Variables|Default|GetP_HP))
  (bind _p_hp_2 (Variables|Default|GetP_HP))
  (bind _returnvalue (* _p_hp_2 0.25))
  (bind _returnvalue_2 (* _p_hp 0.4))
  (|CallParentFunction)
  (Rendering|SetVisibility (Variables|Default|GetParticleSystem3) false false)
  (Transformation|SetWorldScale3D (Variables|Default|GetCylinder) (Math|Vector|MakeVector _returnvalue _returnvalue 0.0))
  (Transformation|SetWorldScale3D (Variables|Default|GetIce_collision) (Math|Vector|MakeVector _returnvalue_2 _returnvalue_2 _returnvalue_2)))