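; WhiteHall is a map object that makes a ThirdPersonCharacter visible again and flags it for a scale change when it enters the collision sphere.
; Tick pins the static mesh and sphere to the mesh's BeginPlay location, forcing fixed scales on both every frame.
; On overlap it matches the other actor against all characters of that class, then shows its mesh and capsule and sets ScaleChange.
; A delayed WarpFlag reset is disconnected and never runs.
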(event OnComponentBeginOverlap(Sphere_Collision)
  (params (OverlappedComponent :type Primitive%20Component%20Object%20Reference) (OtherActor :type Actor%20Object%20Reference) (OtherComp :type Primitive%20Component%20Object%20Reference) (OtherBodyIndex :type Integer) (bFromSweep :type Boolean) (SweepResult :type Hit%20Result%20Structure%20%28by%20ref%29))
  (bind _outactors (Actor|GetAllActorsOfClass "/Game/Revive/Blueprints/Character/ThirdPersonCharacter.ThirdPersonCharacter_C"))
  (for _array_element _outactors
    (if (== _array_element OtherActor)
      (Rendering|SetVisibility (Variables|/Script/Engine.Character|GetMesh _array_element) true false)
      (Rendering|SetVisibility (Variables|/Script/Engine.Character|GetCapsuleComponent _array_element) true false)
      (Variables|/Game/Revive/Blueprints/Character/ThirdPersonCharacter.ThirdPersonCharacter_C|SetScaleChange _array_element true))))

(event EventBeginPlay
  (bind _staticmeshcomponent (Variables|Debug|GetStaticMeshComponent))
  (Variables|Default|SetSetLocation (Transformation|GetWorldLocation _staticmeshcomponent))
  (Variables|Default|SetSetScale (Transformation|GetWorldScale _staticmeshcomponent)))

(event Collision|EventActorBeginOverlap
  (params (OtherActor :type Actor%20Object%20Reference)))

(event EventTick
  (params (DeltaSeconds :type Float%20%28single-precision%29))
  (bind _sphere_collision (Variables|Default|GetSphere_Collision))
  (bind _staticmeshcomponent (Variables|Debug|GetStaticMeshComponent))
  (Utilities|FlowControl|Sequence
    (:then_0
      (Transformation|SetWorldLocation _staticmeshcomponent (Variables|Default|GetSetLocation) false false)
      (Transformation|SetWorldScale3D _staticmeshcomponent "1.000000,1.000000,1.000000")
      (Transformation|SetWorldLocation _sphere_collision (Variables|Default|GetSetLocation) false false)
      (Transformation|SetWorldScale3D _sphere_collision "0.500000,0.500000,0.500000"))))

(fn ConstructionScript)