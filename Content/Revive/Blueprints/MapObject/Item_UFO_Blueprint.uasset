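; UFO map object that serves as the level's clear check, based on how many items the player carries.
; Tick compares the ThirdPersonCharacter's Item count to CLEARITEM and, when reached, sends CLEARBPIFMessage to OtherActor.
; BeginPlay initialises the HP number widget and values.
; Sphere overlap handlers do nothing after their class check, and the HP ratio, camera-facing gauge and hit-message logic are left disconnected.
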(event OnComponentBeginOverlap(Sphere)
  (params (OverlappedComponent :type Primitive%20Component%20Object%20Reference) (OtherActor :type Actor%20Object%20Reference) (OtherComp :type Primitive%20Component%20Object%20Reference) (OtherBodyIndex :type Integer) (bFromSweep :type Boolean) (SweepResult :type Hit%20Result%20Structure%20%28by%20ref%29))
  ;[1 1 1] プレイヤーとの当たり判定（放出・吸収用）
  (if (== (Utilities|GetClass OtherActor) "/Game/Revive/Blueprints/Character/ThirdPersonCharacter.ThirdPersonCharacter_C")
    _))

(event OnComponentEndOverlap(Sphere)
  (params (OverlappedComponent :type Primitive%20Component%20Object%20Reference) (OtherActor :type Actor%20Object%20Reference) (OtherComp :type Primitive%20Component%20Object%20Reference) (OtherBodyIndex :type Integer))
  ;[1 1 1] プレイヤーとの当たり判定（放出・吸収用）
  (if (== (Utilities|GetClass OtherActor) "/Game/Revive/Blueprints/Character/ThirdPersonCharacter.ThirdPersonCharacter_C")
    _))

(event EventBeginPlay
  (bind _ashp_visible_ui (Utilities|Casting|CastToHP_Visible_UI (UserInterface|GetUserWidgetObject (Variables|Default|GetHP_Visibli))))
  (bind _output_get (Variables|Default|SetHP_NUMBER _ashp_visible_ui))
  (Variables|/Game/Revive/Blueprints/UI/HP_Visible_UI.HP_Visible_UI_C|SetHP _output_get (Variables|Default|GetU_MaxHp))
  (Variables|Default|SetU_Hp 0.0)
  (Variables|Default|SetU_MaxHp (Variables|Default|GetU_MaxHp)))

(event Collision|EventActorBeginOverlap
  (params (OtherActor :type Actor%20Object%20Reference)))

(event EventTick
  (params (DeltaSeconds :type Float%20%28single-precision%29))
  ;[1 1 1] CLEAR_ITEMを超える数アイテムを持っている状態で触れるとクリア
  (Utilities|FlowControl|Sequence
    (:then_2
      (if (>= (Variables|/Game/Revive/Blueprints/Character/ThirdPersonCharacter.ThirdPersonCharacter_C|GetItem (.AsThird%20Person%20Character (Utilities|Casting|CastToThirdPersonCharacter (Game|GetPlayerCharacter 0)))) (Variables|Default|GetCLEAR_ITEM))
        (Class|ClearBPIF|CLEARBPIF(Message) (stale OnComponentBeginOverlap(Sphere) OtherActor))))))

(fn ConstructionScript)