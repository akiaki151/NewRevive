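; Child planet map-object Blueprint (Kouris) with a blast zone that affects fire objects entering it.
; Each tick it scales the Bakuha component to half of PHP and prints that size for debugging.
; When a FireOBJ_BP begins overlapping Bakuha, it sets that object's HitIce flag and prints a debug message.
; An HP-based material and particle switch exists but is unwired and never runs.
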(event OnComponentBeginOverlap(bakuha)
  (params (OverlappedComponent :type Primitive%20Component%20Object%20Reference) (OtherActor :type Actor%20Object%20Reference) (OtherComp :type Primitive%20Component%20Object%20Reference) (OtherBodyIndex :type Integer) (bFromSweep :type Boolean) (SweepResult :type Hit%20Result%20Structure%20%28by%20ref%29))
  ;[1 1 1] 貴様（☆）を焼く
  (if (== (Utilities|GetClass OtherActor) "/Game/ThirdPersonBP/Blueprints/FireOBJ_BP.FireOBJ_BP_C")
    (Variables|/Game/ThirdPersonBP/Blueprints/FireOBJ_BP.FireOBJ_BP_C|SetHit_Ice (.AsFire%20OBJ%20BP (Utilities|Casting|CastToFireOBJ_BP OtherActor)) true)
    (Development|PrintString "今貴様は俺の熱風を食らっている" true true "(R=0.000000,G=0.660000,B=1.000000,A=1.000000)" 1.0)))

(event EventBeginPlay
  (|CallParentFunction) ; This node is disabled and will not be called.\nDrag off pins to build functionality.
)

(event Collision|EventActorBeginOverlap
  (params (OtherActor :type Actor%20Object%20Reference))
  (|CallParentFunction OtherActor) ; This node is disabled and will not be called.\nDrag off pins to build functionality.
)

(event EventTick
  (params (DeltaSeconds :type Float%20%28single-precision%29))
  (|CallParentFunction DeltaSeconds)
  (Utilities|FlowControl|Sequence
    (:then_1
      (bind _output_get (Variables|Default|SetBakuhaHanni (Math|Conversions|ToVector(Float) (* (Variables|Default|GetP_HP) 0.5))))
      (Transformation|SetWorldScale3D (Variables|Default|Getbakuha) _output_get))
    (:then_2
      ;[1 1 1] マテリアル変更
      (Development|PrintString (Utilities|String|ToString(Vector) (Variables|Default|GetBakuhaHanni)) true true "(R=1.000000,G=0.390609,B=0.023077,A=1.000000)" 0.0))))

(fn ConstructionScript)