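; Breakable rock wall map object that destroys itself through HitCall when hit by an explosion.
; Its construction script gives each of eight meshes a random one of three rock materials, then snaps the actor to an upper or lower height based on UpdownJudge.
; UP and DOWN overlap volumes detect Copy_Blueprint actors and toggle two player-character flags, NotUpDown and NotUpDown2, to block vertical movement input while something is above or below.
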(event OnComponentEndOverlap(UP)
  (params (OverlappedComponent :type Primitive%20Component%20Object%20Reference) (OtherActor :type Actor%20Object%20Reference) (OtherComp :type Primitive%20Component%20Object%20Reference) (OtherBodyIndex :type Integer))
  (bind _returnvalue (Game|GetPlayerCharacter 0))
  (bind _asthird_person_character (Utilities|Casting|CastToThirdPersonCharacter _returnvalue))
  ;[1 1 1] 上もしくは下にものがあるときは上下移動ボタンを押せなくする
  (if (== (Utilities|GetClass OtherActor) "/Game/Revive/Blueprints/Character/Copy_Blueprint.Copy_Blueprint_C")
    (if (Variables|/Game/Revive/Blueprints/Character/ThirdPersonCharacter.ThirdPersonCharacter_C|GetNot%20Up%20Down _asthird_person_character)
      (Variables|/Game/Revive/Blueprints/Character/ThirdPersonCharacter.ThirdPersonCharacter_C|SetNot%20Up%20Down _asthird_person_character false)
      (else
        (Variables|/Game/Revive/Blueprints/Character/ThirdPersonCharacter.ThirdPersonCharacter_C|SetNotUpDown2 _asthird_person_character false)))))

(event OnComponentBeginOverlap(UP)
  (params (OverlappedComponent :type Primitive%20Component%20Object%20Reference) (OtherActor :type Actor%20Object%20Reference) (OtherComp :type Primitive%20Component%20Object%20Reference) (OtherBodyIndex :type Integer) (bFromSweep :type Boolean) (SweepResult :type Hit%20Result%20Structure%20%28by%20ref%29))
  (bind _returnvalue (Game|GetPlayerCharacter 0))
  (bind _asthird_person_character (Utilities|Casting|CastToThirdPersonCharacter _returnvalue))
  ;[1 1 1] 上もしくは下にものがあるときは上下移動ボタンを押せなくする
  (if (== (Utilities|GetClass OtherActor) "/Game/Revive/Blueprints/Character/Copy_Blueprint.Copy_Blueprint_C")
    (if (Variables|/Game/Revive/Blueprints/Character/ThirdPersonCharacter.ThirdPersonCharacter_C|GetNot%20Up%20Down _asthird_person_character)
      (Variables|/Game/Revive/Blueprints/Character/ThirdPersonCharacter.ThirdPersonCharacter_C|SetNotUpDown2 _asthird_person_character true)
      (else
        (Variables|/Game/Revive/Blueprints/Character/ThirdPersonCharacter.ThirdPersonCharacter_C|SetNot%20Up%20Down _asthird_person_character true)))))

(event OnComponentBeginOverlap(DOWN)
  (params (OverlappedComponent :type Primitive%20Component%20Object%20Reference) (OtherActor :type Actor%20Object%20Reference) (OtherComp :type Primitive%20Component%20Object%20Reference) (OtherBodyIndex :type Integer) (bFromSweep :type Boolean) (SweepResult :type Hit%20Result%20Structure%20%28by%20ref%29))
  (bind _returnvalue (Game|GetPlayerCharacter 0))
  (bind _asthird_person_character (Utilities|Casting|CastToThirdPersonCharacter _returnvalue))
  ;[1 1 1] 上もしくは下にものがあるときは上下移動ボタンを押せなくする
  (if (== (Utilities|GetClass OtherActor) "/Game/Revive/Blueprints/Character/Copy_Blueprint.Copy_Blueprint_C")
    (if (Variables|/Game/Revive/Blueprints/Character/ThirdPersonCharacter.ThirdPersonCharacter_C|GetNot%20Up%20Down _asthird_person_character)
      (Variables|/Game/Revive/Blueprints/Character/ThirdPersonCharacter.ThirdPersonCharacter_C|SetNotUpDown2 _asthird_person_character true)
      (else
        (Variables|/Game/Revive/Blueprints/Character/ThirdPersonCharacter.ThirdPersonCharacter_C|SetNot%20Up%20Down _asthird_person_character true)))))

(event OnComponentEndOverlap(DOWN)
  (params (OverlappedComponent :type Primitive%20Component%20Object%20Reference) (OtherActor :type Actor%20Object%20Reference) (OtherComp :type Primitive%20Component%20Object%20Reference) (OtherBodyIndex :type Integer))
  (bind _returnvalue (Game|GetPlayerCharacter 0))
  (bind _asthird_person_character (Utilities|Casting|CastToThirdPersonCharacter _returnvalue))
  ;[1 1 1] 上もしくは下にものがあるときは上下移動ボタンを押せなくする
  (if (== (Utilities|GetClass OtherActor) "/Game/Revive/Blueprints/Character/Copy_Blueprint.Copy_Blueprint_C")
    (if (Variables|/Game/Revive/Blueprints/Character/ThirdPersonCharacter.ThirdPersonCharacter_C|GetNot%20Up%20Down _asthird_person_character)
      (Variables|/Game/Revive/Blueprints/Character/ThirdPersonCharacter.ThirdPersonCharacter_C|SetNot%20Up%20Down _asthird_person_character false)
      (else
        (Variables|/Game/Revive/Blueprints/Character/ThirdPersonCharacter.ThirdPersonCharacter_C|SetNotUpDown2 _asthird_person_character false)))))

(event EventHitCall
  (params (hitflag :type Boolean))
  ;[1 1 1] 爆発に当たったら消滅させる
  (Actor|DestroyActor))

(fn ConstructionScript
  (bind _returnvalue (Transformation|GetActorLocation))
  (bind _staticmesh2 (Variables|Default|GetStaticMesh2))
  (bind _staticmesh3 (Variables|Default|GetStaticMesh3))
  (bind _staticmesh4 (Variables|Default|GetStaticMesh4))
  (bind _staticmesh5 (Variables|Default|GetStaticMesh5))
  (bind _staticmesh6 (Variables|Default|GetStaticMesh6))
  (bind _staticmesh7 (Variables|Default|GetStaticMesh7))
  (bind _staticmesh1 (Variables|Default|GetStaticMesh1))
  (bind _cube (Variables|Default|GetCube))
  (switch int (Math|Random|RandomIntegerinRange 0 2)
    (:0
      (Rendering|Material|SetMaterial _cube 0 "/Game/Revive/Material/DebriMaterial1/RockFace_MAT.RockFace_MAT"))
    (:1
      (Rendering|Material|SetMaterial _cube 0 "/Game/Revive/Material/DebriMaterial2/Rock_Cliff_MAT.Rock_Cliff_MAT"))
    (:2
      (Rendering|Material|SetMaterial _cube 0 "/Game/Revive/Material/DebriMaterial3/Cliff_Sharp_MAT.Cliff_Sharp_MAT")))
  (switch int (Math|Random|RandomIntegerinRange 0 2)
    (:0
      (Rendering|Material|SetMaterial _staticmesh1 0 "/Game/Revive/Material/DebriMaterial1/RockFace_MAT.RockFace_MAT"))
    (:1
      (Rendering|Material|SetMaterial _staticmesh1 0 "/Game/Revive/Material/DebriMaterial2/Rock_Cliff_MAT.Rock_Cliff_MAT"))
    (:2
      (Rendering|Material|SetMaterial _staticmesh1 0 "/Game/Revive/Material/DebriMaterial3/Cliff_Sharp_MAT.Cliff_Sharp_MAT")))
  (switch int (Math|Random|RandomIntegerinRange 0 2)
    (:0
      (Rendering|Material|SetMaterial _staticmesh2 0 "/Game/Revive/Material/DebriMaterial1/RockFace_MAT.RockFace_MAT"))
    (:1
      (Rendering|Material|SetMaterial _staticmesh2 0 "/Game/Revive/Material/DebriMaterial2/Rock_Cliff_MAT.Rock_Cliff_MAT"))
    (:2
      (Rendering|Material|SetMaterial _staticmesh2 0 "/Game/Revive/Material/DebriMaterial3/Cliff_Sharp_MAT.Cliff_Sharp_MAT")))
  (switch int (Math|Random|RandomIntegerinRange 0 2)
    (:0
      (Rendering|Material|SetMaterial _staticmesh3 0 "/Game/Revive/Material/DebriMaterial1/RockFace_MAT.RockFace_MAT"))
    (:1
      (Rendering|Material|SetMaterial _staticmesh3 0 "/Game/Revive/Material/DebriMaterial2/Rock_Cliff_MAT.Rock_Cliff_MAT"))
    (:2
      (Rendering|Material|SetMaterial _staticmesh3 0 "/Game/Revive/Material/DebriMaterial3/Cliff_Sharp_MAT.Cliff_Sharp_MAT")))
  (switch int (Math|Random|RandomIntegerinRange 0 2)
    (:0
      (Rendering|Material|SetMaterial _staticmesh4 0 "/Game/Revive/Material/DebriMaterial1/RockFace_MAT.RockFace_MAT"))
    (:1
      (Rendering|Material|SetMaterial _staticmesh4 0 "/Game/Revive/Material/DebriMaterial2/Rock_Cliff_MAT.Rock_Cliff_MAT"))
    (:2
      (Rendering|Material|SetMaterial _staticmesh4 0 "/Game/Revive/Material/DebriMaterial3/Cliff_Sharp_MAT.Cliff_Sharp_MAT")))
  (switch int (Math|Random|RandomIntegerinRange 0 2)
    (:0
      (Rendering|Material|SetMaterial _staticmesh5 0 "/Game/Revive/Material/DebriMaterial1/RockFace_MAT.RockFace_MAT"))
    (:1
      (Rendering|Material|SetMaterial _staticmesh5 0 "/Game/Revive/Material/DebriMaterial2/Rock_Cliff_MAT.Rock_Cliff_MAT"))
    (:2
      (Rendering|Material|SetMaterial _staticmesh5 0 "/Game/Revive/Material/DebriMaterial3/Cliff_Sharp_MAT.Cliff_Sharp_MAT")))
  (switch int (Math|Random|RandomIntegerinRange 0 2)
    (:0
      (Rendering|Material|SetMaterial _staticmesh6 0 "/Game/Revive/Material/DebriMaterial1/RockFace_MAT.RockFace_MAT"))
    (:1
      (Rendering|Material|SetMaterial _staticmesh6 0 "/Game/Revive/Material/DebriMaterial2/Rock_Cliff_MAT.Rock_Cliff_MAT"))
    (:2
      (Rendering|Material|SetMaterial _staticmesh6 0 "/Game/Revive/Material/DebriMaterial3/Cliff_Sharp_MAT.Cliff_Sharp_MAT")))
  (switch int (Math|Random|RandomIntegerinRange 0 2)
    (:0
      (Rendering|Material|SetMaterial _staticmesh7 0 "/Game/Revive/Material/DebriMaterial1/RockFace_MAT.RockFace_MAT"))
    (:1
      (Rendering|Material|SetMaterial _staticmesh7 0 "/Game/Revive/Material/DebriMaterial2/Rock_Cliff_MAT.Rock_Cliff_MAT"))
    (:2
      (Rendering|Material|SetMaterial _staticmesh7 0 "/Game/Revive/Material/DebriMaterial3/Cliff_Sharp_MAT.Cliff_Sharp_MAT")))
  (if (Variables|Default|GetUpdown%20Judge)
    (Variables|Default|SetZ_Location 9.2e+02)
    (else
      (Variables|Default|SetZ_Location 3e+01)))
  (Transformation|SetActorLocation (Math|Vector|MakeVector (.x _returnvalue) (.y _returnvalue) (Variables|Default|GetZ_Location)) false false))