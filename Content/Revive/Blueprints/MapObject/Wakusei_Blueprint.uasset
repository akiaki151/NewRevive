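; Planet actor whose HP the player drains or refills as energy while in range and line-hit.
; Tick scales mesh and collision from HP, updates camera-facing HP widgets, and drives line-hit, fire and ice particles.
; Inside an axis zone it orbits its start position until blocked.
; Interface events handle black/white-hole state and teleporting, while UP/DOWN triggers flag the player's vertical-move lock when a Copy_Blueprint overlaps.
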(event OnComponentEndOverlap(UP)
  (params (OverlappedComponent :type Primitive%20Component%20Object%20Reference) (OtherActor :type Actor%20Object%20Reference) (OtherComp :type Primitive%20Component%20Object%20Reference) (OtherBodyIndex :type Integer))
  (bind _returnvalue (Game|GetPlayerCharacter 0))
  (bind _asthird_person_character (Utilities|Casting|CastToThirdPersonCharacter _returnvalue))
  ;[1 1 1] 上もしくは下にものがあるときは上下移動ボタンを押せなくする
  (if (== (Utilities|GetClass OtherActor) "/Game/Revive/Blueprints/Character/Copy_Blueprint.Copy_Blueprint_C")
    (if (Variables|/Game/Revive/Blueprints/Character/ThirdPersonCharacter.ThirdPersonCharacter_C|GetNot%20Up%20Down _asthird_person_character)
      (Variables|/Game/Revive/Blueprints/Character/ThirdPersonCharacter.ThirdPersonCharacter_C|SetNotUpDown2 _asthird_person_character false)
      (Variables|/Game/Revive/Blueprints/Character/ThirdPersonCharacter.ThirdPersonCharacter_C|SetNot%20Up%20Down _asthird_person_character false)
      (else
        (Variables|/Game/Revive/Blueprints/Character/ThirdPersonCharacter.ThirdPersonCharacter_C|SetNotUpDown2 _asthird_person_character false)
        (Variables|/Game/Revive/Blueprints/Character/ThirdPersonCharacter.ThirdPersonCharacter_C|SetNot%20Up%20Down _asthird_person_character false)))))

(event OnComponentBeginOverlap(Playerhit)
  (params (OverlappedComponent :type Primitive%20Component%20Object%20Reference) (OtherActor :type Actor%20Object%20Reference) (OtherComp :type Primitive%20Component%20Object%20Reference) (OtherBodyIndex :type Integer) (bFromSweep :type Boolean) (SweepResult :type Hit%20Result%20Structure%20%28by%20ref%29))
  ;[1 1 1] プレイヤーとの当たり判定（放出・吸収用）
  (if (not (Variables|Default|GetIceFlag))
    (Utilities|FlowControl|Sequence
      (:then_0
        (if (== (Utilities|GetClass OtherActor) "/Game/Revive/Blueprints/Character/ThirdPersonCharacter.ThirdPersonCharacter_C")
          (if (Components|ComponentHasTag OtherComp "PLAYER")
            (if (not (Variables|Default|GetPlayer_In))
              (Variables|Default|SetPlayer_In true))))))))

(event OnComponentEndOverlap(Playerhit)
  (params (OverlappedComponent :type Primitive%20Component%20Object%20Reference) (OtherActor :type Actor%20Object%20Reference) (OtherComp :type Primitive%20Component%20Object%20Reference) (OtherBodyIndex :type Integer))
  ;[1 1 1] プレイヤーとの当たり判定（放出・吸収用）
  (if (== (Utilities|GetClass OtherActor) "/Game/Revive/Blueprints/Character/ThirdPersonCharacter.ThirdPersonCharacter_C")
    (if (Components|ComponentHasTag OtherComp "PLAYER")
      (Variables|Default|SetPlayer_In false))))

(event OnComponentBeginOverlap(UP)
  (params (OverlappedComponent :type Primitive%20Component%20Object%20Reference) (OtherActor :type Actor%20Object%20Reference) (OtherComp :type Primitive%20Component%20Object%20Reference) (OtherBodyIndex :type Integer) (bFromSweep :type Boolean) (SweepResult :type Hit%20Result%20Structure%20%28by%20ref%29))
  (bind _returnvalue (Game|GetPlayerCharacter 0))
  (bind _asthird_person_character (Utilities|Casting|CastToThirdPersonCharacter _returnvalue))
  ;[1 1 1] 上もしくは下にものがあるときは上下移動ボタンを押せなくする
  (if (== (Utilities|GetClass OtherActor) "/Game/Revive/Blueprints/Character/Copy_Blueprint.Copy_Blueprint_C")
    (if (Variables|/Game/Revive/Blueprints/Character/ThirdPersonCharacter.ThirdPersonCharacter_C|GetNot%20Up%20Down _asthird_person_character)
      (Variables|/Game/Revive/Blueprints/Character/ThirdPersonCharacter.ThirdPersonCharacter_C|SetNotUpDown2 _asthird_person_character true)
      (else
        (Variables|/Game/Revive/Blueprints/Character/ThirdPersonCharacter.ThirdPersonCharacter_C|SetNot%20Up%20Down _asthird_person_character true)))))

(event OnComponentBeginOverlap(Sphere2)
  (params (OverlappedComponent :type Primitive%20Component%20Object%20Reference) (OtherActor :type Actor%20Object%20Reference) (OtherComp :type Primitive%20Component%20Object%20Reference) (OtherBodyIndex :type Integer) (bFromSweep :type Boolean) (SweepResult :type Hit%20Result%20Structure%20%28by%20ref%29))
  ;[1 1 1] 回転中に当たったらほしの動きを止める
)

(event OnComponentBeginOverlap(DOWN)
  (params (OverlappedComponent :type Primitive%20Component%20Object%20Reference) (OtherActor :type Actor%20Object%20Reference) (OtherComp :type Primitive%20Component%20Object%20Reference) (OtherBodyIndex :type Integer) (bFromSweep :type Boolean) (SweepResult :type Hit%20Result%20Structure%20%28by%20ref%29))
  (bind _returnvalue (Game|GetPlayerCharacter 0))
  (bind _asthird_person_character (Utilities|Casting|CastToThirdPersonCharacter _returnvalue))
  ;[1 1 1] 上もしくは下にものがあるときは上下移動ボタンを押せなくする
  (if (== (Utilities|GetClass OtherActor) "/Game/Revive/Blueprints/Character/Copy_Blueprint.Copy_Blueprint_C")
    (if (Variables|/Game/Revive/Blueprints/Character/ThirdPersonCharacter.ThirdPersonCharacter_C|GetNot%20Up%20Down _asthird_person_character)
      (Variables|/Game/Revive/Blueprints/Character/ThirdPersonCharacter.ThirdPersonCharacter_C|SetNotUpDown2 _asthird_person_character true)
      (else
        (Variables|/Game/Revive/Blueprints/Character/ThirdPersonCharacter.ThirdPersonCharacter_C|SetNot%20Up%20Down _asthird_person_character true)))))

(event OnComponentEndOverlap(DOWN)
  (params (OverlappedComponent :type Primitive%20Component%20Object%20Reference) (OtherActor :type Actor%20Object%20Reference) (OtherComp :type Primitive%20Component%20Object%20Reference) (OtherBodyIndex :type Integer))
  (bind _returnvalue (Game|GetPlayerCharacter 0))
  (bind _asthird_person_character (Utilities|Casting|CastToThirdPersonCharacter _returnvalue))
  ;[1 1 1] 上もしくは下にものがあるときは上下移動ボタンを押せなくする
  (if (== (Utilities|GetClass OtherActor) "/Game/Revive/Blueprints/Character/Copy_Blueprint.Copy_Blueprint_C")
    (if (Variables|/Game/Revive/Blueprints/Character/ThirdPersonCharacter.ThirdPersonCharacter_C|GetNot%20Up%20Down _asthird_person_character)
      (Variables|/Game/Revive/Blueprints/Character/ThirdPersonCharacter.ThirdPersonCharacter_C|SetNot%20Up%20Down _asthird_person_character false)
      (else
        (Variables|/Game/Revive/Blueprints/Character/ThirdPersonCharacter.ThirdPersonCharacter_C|SetNotUpDown2 _asthird_person_character false)))))

(event Custom|CustomEvent
  (params (hitflag :type Boolean))
  ;[1 1 1] 上もしくは下にものがあるときは上下移動ボタンを押せなくする
  (Utilities|FlowControl|DoOnce false
    (:Completed
      (Actor|DestroyActor))))

(event EventBHBPIF
  (params (Location :type Vector :default "0, 0, 0"))
  (Transformation|SetActorLocation Location false false)
  (Variables|Default|SetWhiteHoleFlag true)
  (Variables|Default|SetBlackHoleFlag false))

(event EventBHBPIF2
  (params (LOCATION :type Vector :default "0, 0, 0"))
  (bind _staticmeshcomponent (Variables|Debug|GetStaticMeshComponent))
  (bind _returnvalue (Transformation|GetWorldLocation _staticmeshcomponent))
  (bind _returnvalue_2 (- LOCATION _returnvalue))
  (Variables|Default|SetBlackHoleFlag true)
  (bind _output_get (Variables|Default|SetBHMove (Math|Vector|Normalize _returnvalue_2))) ; 移動ベクトルセット
  (Variables|Default|SetBHMove (Math|Vector|MakeVector (.x _output_get) (.y _output_get) 0.0)) ; Z軸を０に
  (Variables|Default|SetLength (Math|Vector|VectorLength _returnvalue_2)))

(event EventZikuHanni
  (params (flag :type Boolean) (location :type Vector :default "0, 0, 0") (Component :type Static%20Mesh%20Component%20Object%20Reference))
  ;[1 1 1] 回転する軸に入ってたらtrue
  (Variables|Default|SetZiku_In flag)
  (Variables|Default|SetRotationMove location))

(event EventWakuseiHpDown
  ;[1 1 1] 吸い込まれたときの処理
  (if (Variables|Default|Getplayer_hit)
    (if (Variables|Default|GetPlayer_In)
      (bind _output_get (Variables|Default|SetP_HP (- (Variables|Default|GetP_HP) (Variables|Default|Gethp_add))))
      (Variables|Default|SetP_TIME_MAXHP _output_get))))

(event EventWakuseiHpAdd
  (bind _p_maxhp (Variables|Default|GetP_MAXHP))
  ;[1 1 1] エネルギーを与えられたときの処理
  (if (Variables|Default|Getplayer_hit)
    (if (Variables|Default|GetPlayer_In)
      (if (>= _p_maxhp (Variables|Default|GetP_HP))
        (bind _output_get (Variables|Default|SetP_HP (+ (Variables|Default|GetP_HP) (Variables|Default|Gethp_add))))
        (Variables|Default|SetP_TIME_MAXHP _output_get)
        (bind _asthird_person_character (Utilities|Casting|CastToThirdPersonCharacter (Game|GetPlayerCharacter 0)))
        (Default|HPMINUSOK _asthird_person_character)
        (if (>= (Variables|Default|GetP_HP) _p_maxhp)
          (Audio|Components|Audio|Stop (Variables|Default|Gethousyutu%20))
          (goto _label Reset)
          (else
            (Utilities|FlowControl|DoOnce false :!label _label
              (:Completed
                (Audio|Components|Audio|Play (Variables|Default|Gethousyutu%20) 0.0)))))))))

(event EventLineHit
  (params (flag :type Boolean))
  ;[1 1 1] BPIF取得
  (Variables|Default|Setplayer_hit flag))

(event EventBeginPlay
  (bind _returnvalue (Transformation|GetActorLocation))
  (bind _p_hp (Variables|Default|GetP_HP))
  ;[1 1 1] BeginPlay
  (bind _ashp_ui (Utilities|Casting|CastToHP_UI (UserInterface|GetUserWidgetObject (Variables|Default|GetHP))))
  (bind _output_get (Variables|Default|SetHP_UI _ashp_ui))
  (Variables|/Game/Revive/Blueprints/UI/HP_UI.HP_UI_C|SetHP _output_get 1.0)
  (bind _ashp_visible_ui (Utilities|Casting|CastToHP_Visible_UI (UserInterface|GetUserWidgetObject (Variables|Default|GetHP_Visibli))))
  (bind _output_get_2 (Variables|Default|SetHP_NUMBER _ashp_visible_ui))
  (Variables|/Game/Revive/Blueprints/UI/HP_Visible_UI.HP_Visible_UI_C|SetHP _output_get_2 _p_hp)
  (Variables|Default|SetP_TIME_MAXHP _p_hp)
  (Components|Activation|Deactivate (Variables|Default|GetParticleSystem)) ; パーティクル停止
  (Components|Activation|Deactivate (Variables|Default|GetParticleSystem1)) ; パーティクル停止
  (Variables|Default|SetStartPosition (Math|Vector|MakeVector (.x _returnvalue) (.y _returnvalue) (.z _returnvalue)))
  (Variables|Default|SetP_TIMEHP (Variables|Default|GetP_HP))
  (Audio|Components|Audio|Stop (Variables|Default|Gethousyutu%20)))

(event EventSUIKOMIHIT
  (params (Flag :type Boolean))
  (Variables|Default|SetSUIKOMI Flag))

(event EventHitCall
  (params (hitflag :type Boolean))
  ;[1 1 1] 上もしくは下にものがあるときは上下移動ボタンを押せなくする
  (Utilities|FlowControl|DoOnce false
    (:Completed
      (Actor|DestroyActor))))

(event EventTick
  (params (DeltaSeconds :type Float%20%28single-precision%29))
  (bind _p_hp (Variables|Default|GetP_HP))
  (bind _sphere1 (Variables|Default|GetSphere1))
  (bind _particlesystem2 (Variables|Default|GetParticleSystem2))
  (bind _particlesystem3 (Variables|Default|GetParticleSystem3))
  (bind _staticmeshcomponent (Variables|Debug|GetStaticMeshComponent))
  (bind _returnvalue (* _p_hp 0.07))
  (bind _returnvalue_2 (Math|Float|Absolute(Float) _returnvalue))
  (bind _returnvalue_3 (Math|Conversions|ToVector(Float) _returnvalue_2))
  ;[1 1 1 1 36] Tick
  (Development|PrintString (Utilities|String|ToString(Boolean) (Variables|Default|GetPlayer_In)) true true "(R=0.890206,G=1.000000,B=0.883538,A=1.000000)" 0.0)
  (Utilities|FlowControl|Sequence
    (:then_0
      ;;[1 1 1] HPゲージが常にカメラを向くように設定
      (|CameraMove))
    (:then_1
      ;;[1 1 1] HPの割合を求める
      (|HP＿WARIAI))
    (:then_2
      ;;[1 1 1] パーティクルON/OFF
      (|Particle))
    (:then_3
      ;;[1 1 1] 当たり判定の大きさ
      (if (> (Variables|Default|GetP_HP) 0.0)
        (bind _output_get (Variables|Default|Setscale_float _returnvalue_2))
        (if (>= _output_get 4.0)
          (Transformation|SetWorldScale3D _staticmeshcomponent "4.000000,4.000000,4.000000") ; 大きさが3以上だったら３にする
          (Transformation|SetWorldScale3D _sphere1 "4.000000,4.000000,4.000000")
          (elif (>= 1.5 _output_get)
            (Transformation|SetWorldScale3D _staticmeshcomponent "1.500000,1.500000,1.500000") ; 大きさが3以上だったら３にする
            (Transformation|SetWorldScale3D _sphere1 "1.500000,1.500000,1.500000")
            (else
              (Transformation|SetWorldScale3D _staticmeshcomponent _returnvalue_3)
              (Development|PrintString (Utilities|String|ToString(Vector) _returnvalue_3) true true "(R=0.744709,G=1.000000,B=0.000000,A=1.000000)" 0.0)
              ;;;[1 1 1] コリジョン大きさ変更
              (Transformation|SetWorldScale3D (Variables|Default|GetSphere) "10.000000,10.000000,10.000000")
              (Transformation|SetWorldScale3D (Variables|Default|GetSphere1) _returnvalue_3)
              (Transformation|SetWorldScale3D (Variables|Default|GetHP) "2.500000,2.500000,2.500000")
              (Transformation|SetWorldScale3D (Variables|Default|GetPlayerhit) (Utilities|DEFINEWAKUSEILINEHITSCALE))
              (Transformation|SetWorldScale3D (Variables|Default|GetAction_Collision) "4.000000,4.000000,4.000000"))))))
    (:then_4
      (Utilities|FlowControl|Sequence
        (:then_0
          ;;[1 1 1] 太陽が当たっているときのパーティクル
          (if (Variables|Default|GetFireFlag)
            (if (not (Variables|Default|GetIceFlag))
              (Utilities|FlowControl|DoOnce false :!label _label
                (:Completed
                  (Rendering|SetVisibility (Variables|Default|GetParticleSystem2) true false)
                  (Components|Activation|Activate (Variables|Default|GetParticleSystem2) false) ; パーティクル再生
                  (Utilities|FlowControl|Delay 0.5)
                  (Components|Activation|Deactivate _particlesystem2) ; パーティクル停止
                )))
            (else
              (Components|Activation|Deactivate _particlesystem2) ; パーティクル停止
              (goto _label Reset))))
        (:then_1
          ;;[1 1 1] 軸の範囲に入ったら星の回転
          (if (not (Variables|Default|GetRotationStop))
            (if (not (Variables|Default|GetTutaHit))
              (if (Variables|Default|GetZiku_In)
                (Transformation|AddActorLocalRotation (Variables|Default|GetRotationStarSpeed) false false)
                (bind _output_get_2 (Variables|Default|SetDirectionVector (Math|Rotator|GetRotationXVector (Transformation|GetActorRotation))))
                (Transformation|SetActorLocation (+ (Variables|Default|GetStartPosition) (* (Math|Vector|Normalize _output_get_2) (Variables|Default|GetDistance))) false false)))))
        (:then_2
          ;;[1 1 1] 凍った時の惑星の見た目処理
          (if (Variables|Default|GetIceFlag)
            (if (not (Variables|Default|GetFireFlag))
              (Rendering|SetVisibility (Variables|Default|GetParticleSystem3) true false)
              (Components|Activation|Activate _particlesystem3 false) ; パーティクル再生
              (Transformation|SetWorldLocation _particlesystem3 (Transformation|GetActorLocation) false false))
            (else
              (Components|Activation|Deactivate (Variables|Default|GetParticleSystem3)) ; パーティクル停止
            )))
        (:then_3
          ;[1 1 1] 回転中に当たったらほしの動きを止める
          (if (not (Variables|Default|GetrotationOK?))
            (if (== (Utilities|GetClass (stale OnComponentBeginOverlap(Sphere2) OtherActor)) "/Game/Revive/Blueprints/MapObject/Wakusei_Child_Explosion_BP.Wakusei_Child_Explosion_BP_C")
              (if (Class|PrimitiveComponent|IsOverlappingComponent (Variables|Wakusei_Blueprint_C|GetSphere (.AsWakusei%20Blueprint (Utilities|Casting|CastToWakusei_Blueprint (stale OnComponentBeginOverlap(Sphere2) OtherActor)))) (Variables|Default|GetSphere2)) :!label _label_2
                (Variables|Default|SetRotationStop true)
                (else
                  (Variables|Default|SetRotationStop false)))
              (elif (== (Utilities|GetClass (stale OnComponentBeginOverlap(Sphere2) OtherActor)) "/Game/Revive/Blueprints/MapObject/Wakusei_Infinite_BP.Wakusei_Infinite_BP_C")
                (goto _label_2)))))))
    (:then_5
      (Development|PrintString (Utilities|String|ToString(Boolean) (Variables|Default|GetSUIKOMI)) true true "(R=0.396610,G=0.000000,B=1.000000,A=1.000000)" 0.0))
    (:then_7
      (if (not (Variables|Default|GetIceFlag))
        (if (Variables|Default|GetPlayer_In)
          (if (Variables|Default|Getplayer_hit)
            (if (>= (Variables|Default|GetP_HP) 0.0)
              (bind _asthird_person_character (Utilities|Casting|CastToThirdPersonCharacter (Game|GetPlayerCharacter 0)))
              (if (not (Variables|/Game/Revive/Blueprints/Character/ThirdPersonCharacter.ThirdPersonCharacter_C|GetNoInput _asthird_person_character))
                (if (Variables|/Game/Revive/Blueprints/Character/ThirdPersonCharacter.ThirdPersonCharacter_C|Getline_hit _asthird_person_character)
                  (bind _returnvalue_4 (UserInterface|CreateWidget "/Game/Revive/Blueprints/UI/Suikomi_UI.Suikomi_UI_C"))
                  (UserInterface|Viewport|AddtoViewport _returnvalue_4 0))))))))
    (:then_8
      (if (Variables|Default|GetZiku_In)
        (Collision|SetCollisionEnabled (Variables|Default|Getcolicoli) "QueryAndPhysics")
        (else
          (Collision|SetCollisionEnabled (Variables|Default|Getcolicoli) "NoCollision"))))))

(fn ConstructionScript
  (bind _returnvalue (Transformation|GetActorLocation))
  (bind _p_maxhp (Variables|Default|GetP_MAXHP))
  (bind _staticmeshcomponent (Variables|Debug|GetStaticMeshComponent))
  (bind _returnvalue_2 (* _p_maxhp 0.07))
  (bind _returnvalue_3 (Math|Float|Absolute(Float) _returnvalue_2))
  (bind _returnvalue_4 (Math|Conversions|ToVector(Float) _returnvalue_3))
  (Utilities|FlowControl|Sequence
    (:then_0
      (Transformation|SetWorldScale3D (Variables|Default|Getbakuha) (Variables|Default|GetBakuhaHanni))
      (bind _output_get (Variables|Default|Setscale_float _returnvalue_3))
      (if (>= _output_get 3.0)
        (Transformation|SetWorldScale3D _staticmeshcomponent "3.000000,3.000000,3.000000") ; 大きさが3以上だったら３にする
        (else
          (Transformation|SetWorldScale3D _staticmeshcomponent _returnvalue_4)))
      (Transformation|SetWorldScale3D (Variables|Default|GetSphere) "10.000000,10.000000,10.000000")
      (Transformation|SetWorldScale3D (Variables|Default|GetSphere1) _returnvalue_4)
      (Rendering|SetVisibility (Variables|Default|Getcolicoli) false false)
      (if (Variables|Default|GetUpdown_Judge)
        (Variables|Default|SetZ_Location 1.16e+03)
        (else
          (Variables|Default|SetZ_Location 2.3e+02)))
      (Transformation|SetActorLocation (Math|Vector|MakeVector (.x _returnvalue) (.y _returnvalue) (Variables|Default|GetZ_Location)) false false)
      (Rendering|SetVisibility (Variables|Default|GetParticleSystem3) false false))
    (:then_1
      (Rendering|SetVisibility (Variables|Default|GetSphere1) (Variables|Default|GetSphere1_look) false)
      (Rendering|SetVisibility (Variables|Default|Getbakuha) (Variables|Default|Getbakuha_look) false)
      (Rendering|SetVisibility (Variables|Default|GetSphere) (Variables|Default|Getsphere_look) false)
      (Rendering|SetVisibility (Variables|Default|GetPlayerhit) (Variables|Default|Getplayer_hit_look) false)
      (Rendering|SetVisibility (Variables|Default|GetAction_Collision) (Variables|Default|Getaction_coll_look) false)
      (Rendering|SetVisibility (Variables|Default|GetUP) (Variables|Default|Getup_look) false)
      (Rendering|SetVisibility (Variables|Default|GetDOWN) (Variables|Default|Getdown_look) false))))