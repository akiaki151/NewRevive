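; Child planet map object (Wakusei_Child_Tree_BP) that keeps a fixed size while an attached Tuta_BP vine grows or shrinks along Y with its HP.
; Each tick NewFunction0 rescales and repositions the vine and its Box from PHP/PMAXHP, hiding both at 5% or below.
; A DoOnce starts the vine sound when HP changes between empty and full, stopping it otherwise.
; Tick also zeroes rotation, floors HP at zero and disables Colicoli collision.
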(event EventBeginPlay
  (|CallParentFunction)
  (Transformation|SetWorldScale3D (Variables|Default|GetStaticMeshComponent) "4.000000,4.000000,4.000000") ; 大きさが3以上だったら３にする
  (Audio|Components|Audio|Stop (Variables|Default|Gettuta_SE)))

(event Collision|EventActorBeginOverlap
  (params (OtherActor :type Actor%20Object%20Reference))
  (|CallParentFunction OtherActor) ; This node is disabled and will not be called.\nDrag off pins to build functionality.
)

(event EventTick
  (params (DeltaSeconds :type Float%20%28single-precision%29))
  (|CallParentFunction DeltaSeconds)
  (Utilities|FlowControl|Sequence
    (:then_0
      (if (== (Variables|Default|GetP_HP) (Variables|Default|GetkeepHP_0))
        (CallFunction|NewFunction0)
        (Audio|Components|Audio|Stop (Variables|Default|Gettuta_SE) :!label _label)
        (goto _label_2 Reset)
        (else
          (CallFunction|NewFunction0)
          (if (>= (Variables|Default|GetP_HP) (Variables|Default|GetP_MAXHP))
            (goto _label)
            (elif (>= 0.0 (Variables|Default|GetP_HP))
              (goto _label)
              (else
                (Utilities|FlowControl|DoOnce false :!label _label_2
                  (:Completed
                    (Audio|Components|Audio|Play (Variables|Default|Gettuta_SE) 0.0)))))))))
    (:then_1
      (Transformation|SetActorRotation "0, 0, 0"))
    (:then_2
      (if (<= (Variables|Default|GetP_HP) 0.0)
        (Variables|Default|SetP_HP 0.0)))
    (:then_3
      (Collision|SetCollisionEnabled (Variables|Default|Getcolicoli) "NoCollision"))))

(fn ConstructionScript
  (|CallParentFunction))

(fn NewFunction0
  (bind _childactor (Variables|Default|GetChildActor))
  (bind _childactor_2 (Variables|Default|GetChildActor))
  (bind _p_maxhp (Variables|Default|GetP_MAXHP))
  (bind _p_hp (Variables|Default|GetP_HP))
  (bind _staticmeshcomponent (Variables|Default|GetStaticMeshComponent))
  (bind _p_maxhp_2 (Variables|Default|GetP_MAXHP))
  (bind _returnvalue (/ _p_maxhp 3.0))
  (bind _returnvalue_2 (Transformation|GetWorldLocation _staticmeshcomponent))
  (bind _returnvalue_3 (/ _p_hp _p_maxhp_2))
  (bind _childactor_3 (Variables|/Script/Engine.ChildActorComponent|GetChildActor _childactor))
  (bind _returnvalue_4 (Math|Float|Absolute(Float) _returnvalue_3))
  (bind _returnvalue_5 (Math|Conversions|ToVector(Float) _returnvalue_4))
  (bind _returnvalue_6 (* (.y _returnvalue_5) _returnvalue))
  ;[1 1 1] 当たり判定の大きさ
  (Transformation|SetWorldScale3D (Variables|Default|GetStaticMeshComponent) "4.000000,4.000000,4.000000") ; 星の大きさは固定
  (bind _output_get (Variables|Default|Setscale_float _returnvalue_4))
  (if (<= _output_get 0.05) ; HPが５％以下ならツタ表示しない
    (Transformation|SetWorldScale3D (Variables|/Game/Revive/Blueprints/MapObject/Tuta_BP.Tuta_BP_C|GetBox (.AsTuta%20BP (Utilities|Casting|CastToTuta_BP (Variables|/Script/Engine.ChildActorComponent|GetChildActor _childactor_2)))) "0, 0, 0")
    (Transformation|SetWorldScale3D _childactor_2 "0, 0, 0")
    (else
      (Transformation|SetWorldScale3D (Variables|/Game/Revive/Blueprints/MapObject/Tuta_BP.Tuta_BP_C|GetBox (.AsTuta%20BP (Utilities|Casting|CastToTuta_BP _childactor_3))) (Math|Vector|MakeVector 2.0 _returnvalue_6 2.0))
      (Transformation|SetWorldScale3D _childactor (Math|Vector|MakeVector 0.5 _returnvalue_6 0.5))
      (Transformation|SetActorLocation _childactor_3 (Math|Vector|MakeVector (.x _returnvalue_2) (+ (.y _returnvalue_2) (* (Variables|Default|GetP_HP) 12.0)) (.z _returnvalue_2)) false false)))
  (Transformation|SetWorldScale3D (Variables|Default|GetHP) "2.500000,2.500000,2.500000")
  (Transformation|SetWorldScale3D (Variables|Default|GetSphere) "8.000000,8.000000,8.000000")
  (Transformation|SetWorldScale3D (Variables|Default|GetSphere1) "4.000000,4.000000,4.000000")
  (Variables|Default|SetkeepHP_0 (Variables|Default|GetP_HP)))