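; Wall map object that blocks the player's up/down move button while a Copy_Blueprint actor is above or below it.
; UP and DOWN component overlaps set and clear NotUpDown and NotUpDown2 on the ThirdPersonCharacter, using the pair as a makeshift two-slot overlap counter.
; The construction script snaps the wall to an upper or lower fixed height based on UpdownJudge, keeping its X and Y.
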(event OnComponentBeginOverlap(UP)
  (params (OverlappedComponent :type Primitive%20Component%20Object%20Reference) (OtherActor :type Actor%20Object%20Reference) (OtherComp :type Primitive%20Component%20Object%20Reference) (OtherBodyIndex :type Integer) (bFromSweep :type Boolean) (SweepResult :type Hit%20Result%20Structure%20%28by%20ref%29))
  (bind _returnvalue (Game|GetPlayerCharacter 0))
  (bind _asthird_person_character (Utilities|Casting|CastToThirdPersonCharacter _returnvalue))
  ;[1 1 1] 上もしくは下にものがあるときは上下移動ボタンを押せなくする
  (if (== (Utilities|GetClass OtherActor) "/Game/Revive/Blueprints/Character/Copy_Blueprint.Copy_Blueprint_C")
    (if (Variables|/Game/Revive/Blueprints/Character/ThirdPersonCharacter.ThirdPersonCharacter_C|GetNot%20Up%20Down _asthird_person_character)
      (Variables|/Game/Revive/Blueprints/Character/ThirdPersonCharacter.ThirdPersonCharacter_C|SetNotUpDown2 _asthird_person_character true)
      (else
        (Variables|/Game/Revive/Blueprints/Character/ThirdPersonCharacter.ThirdPersonCharacter_C|SetNot%20Up%20Down _asthird_person_character true)))))

(event OnComponentEndOverlap(UP)
  (params (OverlappedComponent :type Primitive%20Component%20Object%20Reference) (OtherActor :type Actor%20Object%20Reference) (OtherComp :type Primitive%20Component%20Object%20Reference) (OtherBodyIndex :type Integer))
  (bind _returnvalue (Game|GetPlayerCharacter 0))
  (bind _asthird_person_character (Utilities|Casting|CastToThirdPersonCharacter _returnvalue))
  ;[1 1 1] 上もしくは下にものがあるときは上下移動ボタンを押せなくする
  (if (== (Utilities|GetClass OtherActor) "/Game/Revive/Blueprints/Character/Copy_Blueprint.Copy_Blueprint_C")
    (if (Variables|/Game/Revive/Blueprints/Character/ThirdPersonCharacter.ThirdPersonCharacter_C|GetNot%20Up%20Down _asthird_person_character)
      (Variables|/Game/Revive/Blueprints/Character/ThirdPersonCharacter.ThirdPersonCharacter_C|SetNot%20Up%20Down _asthird_person_character false)
      (else
        (Variables|/Game/Revive/Blueprints/Character/ThirdPersonCharacter.ThirdPersonCharacter_C|SetNotUpDown2 _asthird_person_character false)))))

(event OnComponentBeginOverlap(DOWN)
  (params (OverlappedComponent :type Primitive%20Component%20Object%20Reference) (OtherActor :type Actor%20Object%20Reference) (OtherComp :type Primitive%20Component%20Object%20Reference) (OtherBodyIndex :type Integer) (bFromSweep :type Boolean) (SweepResult :type Hit%20Result%20Structure%20%28by%20ref%29))
  (bind _returnvalue (Game|GetPlayerCharacter 0))
  (bind _asthird_person_character (Utilities|Casting|CastToThirdPersonCharacter _returnvalue))
  ;[1 1 1] 上もしくは下にものがあるときは上下移動ボタンを押せなくする
  (if (== (Utilities|GetClass OtherActor) "/Game/Revive/Blueprints/Character/Copy_Blueprint.Copy_Blueprint_C")
    (if (Variables|/Game/Revive/Blueprints/Character/ThirdPersonCharacter.ThirdPersonCharacter_C|GetNot%20Up%20Down _asthird_person_character)
      (Variables|/Game/Revive/Blueprints/Character/ThirdPersonCharacter.ThirdPersonCharacter_C|SetNotUpDown2 _asthird_person_character true)
      (else
        (Variables|/Game/Revive/Blueprints/Character/ThirdPersonCharacter.ThirdPersonCharacter_C|SetNot%20Up%20Down _asthird_person_character true)))))

(event OnComponentEndOverlap(DOWN)
  (params (OverlappedComponent :type Primitive%20Component%20Object%20Reference) (OtherActor :type Actor%20Object%20Reference) (OtherComp :type Primitive%20Component%20Object%20Reference) (OtherBodyIndex :type Integer))
  (bind _returnvalue (Game|GetPlayerCharacter 0))
  (bind _asthird_person_character (Utilities|Casting|CastToThirdPersonCharacter _returnvalue))
  ;[1 1 1] 上もしくは下にものがあるときは上下移動ボタンを押せなくする
  (if (== (Utilities|GetClass OtherActor) "/Game/Revive/Blueprints/Character/Copy_Blueprint.Copy_Blueprint_C")
    (if (Variables|/Game/Revive/Blueprints/Character/ThirdPersonCharacter.ThirdPersonCharacter_C|GetNot%20Up%20Down _asthird_person_character)
      (Variables|/Game/Revive/Blueprints/Character/ThirdPersonCharacter.ThirdPersonCharacter_C|SetNot%20Up%20Down _asthird_person_character false)
      (else
        (Variables|/Game/Revive/Blueprints/Character/ThirdPersonCharacter.ThirdPersonCharacter_C|SetNotUpDown2 _asthird_person_character false)))))

(event EventBeginPlay)

(event Collision|EventActorBeginOverlap
  (params (OtherActor :type Actor%20Object%20Reference)))

(event EventTick
  (params (DeltaSeconds :type Float%20%28single-precision%29)))

(fn ConstructionScript
  (bind _returnvalue (Transformation|GetActorLocation))
  (if (Variables|Default|GetUpdown%20Judge)
    (Variables|Default|SetZ_Location 9.3e+02)
    (else
      (Variables|Default|SetZ_Location 4e+01)))
  (Transformation|SetActorLocation (Math|Vector|MakeVector (.x _returnvalue) (.y _returnvalue) (Variables|Default|GetZ_Location)) false false))