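; Fire planet (Wakusei) map object that spreads fire to normal and energy planets on its UpdownJudge side.
; Each tick it scales its fire range and ring by PHP, writes PHP to overlapping planets and sets their fire/ice flags by comparison with IceGetHp.
; It also toggles flame particles, ring visibility and the Suikomi UI.
; The construction script pre-applies fire without overlap checks and sets Damage to a sentinel that loops skip.
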(event OnComponentEndOverlap(Sphere)
  (params (OverlappedComponent :type Primitive%20Component%20Object%20Reference) (OtherActor :type Actor%20Object%20Reference) (OtherComp :type Primitive%20Component%20Object%20Reference) (OtherBodyIndex :type Integer))
  ;[1 1 1] COLLISION
)

(event EventBeginPlay
  ;[1 1 1] BEGIN
  (|CallParentFunction)
  (Utilities|IsValid "/Game/Revive/Blueprints/MapObject/Wakusei_Child_Ice_BP.Wakusei_Child_Ice_BP"
    (:Is%20Valid
      (Actor|Tick|AddTickPrerequisiteActor 0))))

(event Collision|EventActorBeginOverlap
  (params (OtherActor :type Actor%20Object%20Reference))
  (|CallParentFunction OtherActor) ; This node is disabled and will not be called.\nDrag off pins to build functionality.
)

(event EventTick
  (params (DeltaSeconds :type Float%20%28single-precision%29))
  (bind _p_hp (Variables|Default|GetP_HP))
  (bind _cylinder (Variables|Default|GetCylinder))
  (bind _p_hp_2 (Variables|Default|GetP_HP))
  (bind _flameplanet (Variables|Default|Getflameplanet))
  (bind _returnvalue (* _p_hp_2 0.25))
  (bind _returnvalue_2 (* _p_hp 0.28))
  ;[1 1 1] UPDATE
  (|CallParentFunction DeltaSeconds)
  (Utilities|FlowControl|Sequence
    (:then_1
      (if (Variables|Default|GetPlayer_In)
        (if (Variables|Default|Getplayer_hit)
          (if (>= (Variables|Default|GetP_HP) 0.0)
            (bind _asthird_person_character (Utilities|Casting|CastToThirdPersonCharacter (Game|GetPlayerCharacter 0)))
            (if (not (Variables|/Game/Revive/Blueprints/Character/ThirdPersonCharacter.ThirdPersonCharacter_C|GetNoInput _asthird_person_character))
              (if (Variables|/Game/Revive/Blueprints/Character/ThirdPersonCharacter.ThirdPersonCharacter_C|Getline_hit _asthird_person_character)
                (bind _returnvalue_3 (UserInterface|CreateWidget "/Game/Revive/Blueprints/UI/Suikomi_UI.Suikomi_UI_C"))
                (UserInterface|Viewport|AddtoViewport _returnvalue_3 0)))))))
    (:then_2
      (if (> (Variables|Default|GetP_HP) 0.0)
        (Components|Activation|Activate _flameplanet false) ; パーティクル再生
        (else
          (Components|Activation|Deactivate _flameplanet) ; パーティクル停止
        )))
    (:then_3
      (bind _outactors (Actor|GetAllActorsOfClass "/Game/Revive/Blueprints/MapObject/Wakusei_Blueprint.Wakusei_Blueprint_C"))
      (for _array_element _outactors
        (if (not (Utilities|ClassIsChildOf (Utilities|GetClass _array_element) "Wakusei_Child_Fire_BP_C"))
          (bind _aswakusei_blueprint (Utilities|Casting|CastToWakusei_Blueprint _array_element))
          (if (not (== (Variables|/Game/Revive/Blueprints/MapObject/Wakusei_Blueprint.Wakusei_Blueprint_C|GetDamage _aswakusei_blueprint) 1.41421))
            (if (Class|PrimitiveComponent|IsOverlappingComponent (Variables|Default|GetFire_collision) (Variables|/Game/Revive/Blueprints/MapObject/Wakusei_Blueprint.Wakusei_Blueprint_C|GetSphere1 _aswakusei_blueprint))
              (if (Math|Boolean|Equal(Boolean) (Variables|Default|GetUpdown_Judge) (Variables|/Game/Revive/Blueprints/MapObject/Wakusei_Blueprint.Wakusei_Blueprint_C|GetUpdown_Judge _aswakusei_blueprint))
                (Variables|/Game/Revive/Blueprints/MapObject/Wakusei_Blueprint.Wakusei_Blueprint_C|SetFireGetHp _aswakusei_blueprint (Variables|Default|GetP_HP))
                (if (<= (Variables|/Game/Revive/Blueprints/MapObject/Wakusei_Blueprint.Wakusei_Blueprint_C|GetIceGetHp _aswakusei_blueprint) (Variables|/Game/Revive/Blueprints/MapObject/Wakusei_Blueprint.Wakusei_Blueprint_C|GetFireGetHp _aswakusei_blueprint))
                  (Variables|/Game/Revive/Blueprints/MapObject/Wakusei_Blueprint.Wakusei_Blueprint_C|SetFireFlag _aswakusei_blueprint true)
                  (Variables|/Game/Revive/Blueprints/MapObject/Wakusei_Blueprint.Wakusei_Blueprint_C|SetIceFlag _aswakusei_blueprint false)
                  (Variables|/Game/Revive/Blueprints/MapObject/Wakusei_Blueprint.Wakusei_Blueprint_C|SetIceGetHp _aswakusei_blueprint 0.0)
                  (else
                    (Variables|/Game/Revive/Blueprints/MapObject/Wakusei_Blueprint.Wakusei_Blueprint_C|SetFireFlag _aswakusei_blueprint false)
                    (Variables|/Game/Revive/Blueprints/MapObject/Wakusei_Blueprint.Wakusei_Blueprint_C|SetIceFlag _aswakusei_blueprint true)
                    (Variables|/Game/Revive/Blueprints/MapObject/Wakusei_Blueprint.Wakusei_Blueprint_C|SetFireGetHp _aswakusei_blueprint 0.0)))))))))
    (:then_4
      (bind _outactors_2 (Actor|GetAllActorsOfClass "/Game/Revive/Blueprints/MapObject/EnergieWakusei_Blueprint.EnergieWakusei_Blueprint_C"))
      (for _array_element_2 _outactors_2
        (bind _asenergie_wakusei_blueprint (Utilities|Casting|CastToEnergieWakusei_Blueprint _array_element_2))
        (if (Class|PrimitiveComponent|IsOverlappingComponent (Variables|Default|GetFire_collision) (Variables|/Game/Revive/Blueprints/MapObject/EnergieWakusei_Blueprint.EnergieWakusei_Blueprint_C|GetSphere1 _asenergie_wakusei_blueprint))
          (if (Math|Boolean|Equal(Boolean) (Variables|Default|GetUpdown_Judge) (Variables|/Game/Revive/Blueprints/MapObject/EnergieWakusei_Blueprint.EnergieWakusei_Blueprint_C|GetUpdown_Judge _asenergie_wakusei_blueprint))
            (Variables|/Game/Revive/Blueprints/MapObject/EnergieWakusei_Blueprint.EnergieWakusei_Blueprint_C|SetFireGetHp _asenergie_wakusei_blueprint (Variables|Default|GetP_HP))
            (if (<= (Variables|/Game/Revive/Blueprints/MapObject/EnergieWakusei_Blueprint.EnergieWakusei_Blueprint_C|GetIceGetHp _asenergie_wakusei_blueprint) (Variables|/Game/Revive/Blueprints/MapObject/EnergieWakusei_Blueprint.EnergieWakusei_Blueprint_C|GetFireGetHp _asenergie_wakusei_blueprint))
              (Variables|/Game/Revive/Blueprints/MapObject/EnergieWakusei_Blueprint.EnergieWakusei_Blueprint_C|SetFireFlag _asenergie_wakusei_blueprint true)
              (Variables|/Game/Revive/Blueprints/MapObject/EnergieWakusei_Blueprint.EnergieWakusei_Blueprint_C|SetIceFlag _asenergie_wakusei_blueprint false)
              (Variables|/Game/Revive/Blueprints/MapObject/EnergieWakusei_Blueprint.EnergieWakusei_Blueprint_C|SetIceGetHp _asenergie_wakusei_blueprint 0.0)
              (else
                (Variables|/Game/Revive/Blueprints/MapObject/EnergieWakusei_Blueprint.EnergieWakusei_Blueprint_C|SetFireFlag _asenergie_wakusei_blueprint true)
                (Variables|/Game/Revive/Blueprints/MapObject/EnergieWakusei_Blueprint.EnergieWakusei_Blueprint_C|SetIceFlag _asenergie_wakusei_blueprint true)
                (Variables|/Game/Revive/Blueprints/MapObject/EnergieWakusei_Blueprint.EnergieWakusei_Blueprint_C|SetFireGetHp _asenergie_wakusei_blueprint 0.0)))))))
    (:then_5
      (bind _outactors_3 (Actor|GetAllActorsOfClass "/Game/Revive/Blueprints/Character/ThirdPersonCharacter.ThirdPersonCharacter_C"))
      (for _array_element_3 _outactors_3
        (if (Math|Boolean|Equal(Boolean) (Variables|Default|GetUpdown_Judge) (Variables|/Game/Revive/Blueprints/Character/ThirdPersonCharacter.ThirdPersonCharacter_C|GetPlayerUP _array_element_3))
          (Rendering|SetVisibility _cylinder true false)
          (else
            (Rendering|SetVisibility _cylinder false false)))))
    (:then_6
      (Transformation|SetWorldScale3D (Variables|Default|GetPlayerhit) (Utilities|DEFINEWAKUSEILINEHITSCALE))
      (Transformation|SetWorldScale3D (Variables|Default|GetHP) "2.500000,2.500000,2.500000")
      (Transformation|SetWorldScale3D (Variables|Default|GetCylinder) (Math|Vector|MakeVector _returnvalue _returnvalue 0.0))
      (Transformation|SetWorldScale3D (Variables|Default|GetFire_collision) (Math|Vector|MakeVector _returnvalue_2 _returnvalue_2 _returnvalue_2)))
    (:then_7
      ;[1 1 1] COLLISION
      (Utilities|FlowControl|Sequence
        (:then_0
          ;;[1 1 1] wakuseiがIceWakuseiと当たっていなかったらWakuseiの体力に０を代入する
          (if (Utilities|IsValid (stale OnComponentEndOverlap(Sphere) OtherActor))
            (if (Utilities|ClassIsChildOf (Utilities|GetClass (stale OnComponentEndOverlap(Sphere) OtherActor)) "/Game/Revive/Blueprints/MapObject/Wakusei_Blueprint.Wakusei_Blueprint_C")
              (bind _aswakusei_blueprint_2 (Utilities|Casting|CastToWakusei_Blueprint (stale OnComponentEndOverlap(Sphere) OtherActor)))
              (if (not (Class|PrimitiveComponent|IsOverlappingComponent (Variables|Default|GetFire_collision) (Variables|/Game/Revive/Blueprints/MapObject/Wakusei_Blueprint.Wakusei_Blueprint_C|GetSphere1 _aswakusei_blueprint_2)))
                (Variables|/Game/Revive/Blueprints/MapObject/Wakusei_Blueprint.Wakusei_Blueprint_C|SetFireGetHp _aswakusei_blueprint_2 0.0)))))
        (:then_1
          ;;[1 1 1] EnergiewakuseiがIceWakuseiと当たっていなかったらEnergieWakuseiの体力に０を代入する
          (if (Utilities|ClassIsChildOf (Utilities|GetClass (stale OnComponentEndOverlap(Sphere) OtherActor)) "/Game/Revive/Blueprints/MapObject/EnergieWakusei_Blueprint.EnergieWakusei_Blueprint_C")
            (bind _asenergie_wakusei_blueprint_2 (Utilities|Casting|CastToEnergieWakusei_Blueprint (stale OnComponentEndOverlap(Sphere) OtherActor)))
            (if (not (Class|PrimitiveComponent|IsOverlappingComponent (Variables|Default|GetFire_collision) (Variables|/Game/Revive/Blueprints/MapObject/EnergieWakusei_Blueprint.EnergieWakusei_Blueprint_C|GetSphere1 _asenergie_wakusei_blueprint_2)))
              (Variables|/Game/Revive/Blueprints/MapObject/EnergieWakusei_Blueprint.EnergieWakusei_Blueprint_C|SetFireGetHp _asenergie_wakusei_blueprint_2 0.0))))))))

(fn ConstructionScript
  (bind _p_hp (Variables|Default|GetP_HP))
  (bind _p_hp_2 (Variables|Default|GetP_HP))
  (bind _p_hp_3 (Variables|Default|GetP_HP))
  (bind _returnvalue (* _p_hp_3 0.25))
  (bind _returnvalue_2 (* _p_hp 0.4))
  (bind _returnvalue_3 (* _p_hp_2 0.28))
  (|CallParentFunction)
  (Utilities|FlowControl|Sequence
    (:then_0
      (Rendering|SetVisibility (Variables|Default|GetParticleSystem3) false false)
      (Transformation|SetWorldScale3D (Variables|Default|GetCylinder) (Math|Vector|MakeVector _returnvalue _returnvalue 0.0))
      (Transformation|SetWorldScale3D (Variables|Default|GetFire_collision) (Math|Vector|MakeVector _returnvalue_2 _returnvalue_2 _returnvalue_2))
      (Transformation|SetWorldScale3D (Variables|Default|GetFire_collision) (Math|Vector|MakeVector _returnvalue_3 _returnvalue_3 _returnvalue_3))
      (Variables|Default|SetDamage 1.41421))
    (:then_1
      (bind _outactors (Actor|GetAllActorsOfClass "/Game/Revive/Blueprints/MapObject/Wakusei_Blueprint.Wakusei_Blueprint_C"))
      (for _array_element _outactors
        (if (not (Utilities|ClassIsChildOf (Utilities|GetClass _array_element) "Wakusei_Child_Fire_BP_C"))
          (bind _aswakusei_blueprint (Utilities|Casting|CastToWakusei_Blueprint _array_element))
          (if (not (== (Variables|/Game/Revive/Blueprints/MapObject/Wakusei_Blueprint.Wakusei_Blueprint_C|GetDamage _aswakusei_blueprint) 1.41421))
            (if true
              (if (Math|Boolean|Equal(Boolean) (Variables|Default|GetUpdown_Judge) (Variables|/Game/Revive/Blueprints/MapObject/Wakusei_Blueprint.Wakusei_Blueprint_C|GetUpdown_Judge _aswakusei_blueprint))
                (Variables|/Game/Revive/Blueprints/MapObject/Wakusei_Blueprint.Wakusei_Blueprint_C|SetFireGetHp _aswakusei_blueprint (Variables|Default|GetP_HP))
                (if (<= (Variables|/Game/Revive/Blueprints/MapObject/Wakusei_Blueprint.Wakusei_Blueprint_C|GetIceGetHp _aswakusei_blueprint) (Variables|/Game/Revive/Blueprints/MapObject/Wakusei_Blueprint.Wakusei_Blueprint_C|GetFireGetHp _aswakusei_blueprint))
                  (Variables|/Game/Revive/Blueprints/MapObject/Wakusei_Blueprint.Wakusei_Blueprint_C|SetFireFlag _aswakusei_blueprint true)
                  (Variables|/Game/Revive/Blueprints/MapObject/Wakusei_Blueprint.Wakusei_Blueprint_C|SetIceFlag _aswakusei_blueprint false)
                  (Variables|/Game/Revive/Blueprints/MapObject/Wakusei_Blueprint.Wakusei_Blueprint_C|SetIceGetHp _aswakusei_blueprint 0.0)
                  (Variables|/Game/Revive/Blueprints/MapObject/Wakusei_Blueprint.Wakusei_Blueprint_C|SetFireSE _aswakusei_blueprint true)
                  (else
                    (Variables|/Game/Revive/Blueprints/MapObject/Wakusei_Blueprint.Wakusei_Blueprint_C|SetFireFlag _aswakusei_blueprint false)
                    (Variables|/Game/Revive/Blueprints/MapObject/Wakusei_Blueprint.Wakusei_Blueprint_C|SetIceFlag _aswakusei_blueprint true)
                    (Variables|/Game/Revive/Blueprints/MapObject/Wakusei_Blueprint.Wakusei_Blueprint_C|SetFireGetHp _aswakusei_blueprint 0.0)
                    (Variables|/Game/Revive/Blueprints/MapObject/Wakusei_Blueprint.Wakusei_Blueprint_C|SetIceSE _aswakusei_blueprint true)))))))))
    (:then_2
      (bind _outactors_2 (Actor|GetAllActorsOfClass "/Game/Revive/Blueprints/MapObject/EnergieWakusei_Blueprint.EnergieWakusei_Blueprint_C"))
      (for _array_element_2 _outactors_2
        (bind _asenergie_wakusei_blueprint (Utilities|Casting|CastToEnergieWakusei_Blueprint _array_element_2))
        (if true
          (if (Math|Boolean|Equal(Boolean) (Variables|Default|GetUpdown_Judge) (Variables|/Game/Revive/Blueprints/MapObject/EnergieWakusei_Blueprint.EnergieWakusei_Blueprint_C|GetUpdown_Judge _asenergie_wakusei_blueprint))
            (Variables|/Game/Revive/Blueprints/MapObject/EnergieWakusei_Blueprint.EnergieWakusei_Blueprint_C|SetFireGetHp _asenergie_wakusei_blueprint (Variables|Default|GetP_HP))
            (if (<= (Variables|/Game/Revive/Blueprints/MapObject/EnergieWakusei_Blueprint.EnergieWakusei_Blueprint_C|GetIceGetHp _asenergie_wakusei_blueprint) (Variables|/Game/Revive/Blueprints/MapObject/EnergieWakusei_Blueprint.EnergieWakusei_Blueprint_C|GetFireGetHp _asenergie_wakusei_blueprint))
              (Variables|/Game/Revive/Blueprints/MapObject/EnergieWakusei_Blueprint.EnergieWakusei_Blueprint_C|SetFireFlag _asenergie_wakusei_blueprint true)
              (Variables|/Game/Revive/Blueprints/MapObject/EnergieWakusei_Blueprint.EnergieWakusei_Blueprint_C|SetIceFlag _asenergie_wakusei_blueprint false)
              (Variables|/Game/Revive/Blueprints/MapObject/EnergieWakusei_Blueprint.EnergieWakusei_Blueprint_C|SetIceGetHp _asenergie_wakusei_blueprint 0.0)
              (else
                (Variables|/Game/Revive/Blueprints/MapObject/EnergieWakusei_Blueprint.EnergieWakusei_Blueprint_C|SetFireFlag _asenergie_wakusei_blueprint true)
                (Variables|/Game/Revive/Blueprints/MapObject/EnergieWakusei_Blueprint.EnergieWakusei_Blueprint_C|SetIceFlag _asenergie_wakusei_blueprint true)
                (Variables|/Game/Revive/Blueprints/MapObject/EnergieWakusei_Blueprint.EnergieWakusei_Blueprint_C|SetFireGetHp _asenergie_wakusei_blueprint 0.0)))))))))