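; Energy planet map object whose HP the player can affect within its overlap sphere, showing a suction UI.
; Tick drives mesh scale, camera-facing energy/HP widgets and low-energy particles from HP.
; Fire and ice values select burning or frozen effects, and the planet orbits its start point inside an axis range until the player enters.
; UP/DOWN triggers block player vertical movement near Copy_Blueprint actors, while construction snaps height to one of two levels.
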(event OnComponentEndOverlap(UP)
  (params (OverlappedComponent :type Primitive%20Component%20Object%20Reference) (OtherActor :type Actor%20Object%20Reference) (OtherComp :type Primitive%20Component%20Object%20Reference) (OtherBodyIndex :type Integer))
  (bind _returnvalue (Game|GetPlayerCharacter 0))
  (bind _asthird_person_character (Utilities|Casting|CastToThirdPersonCharacter _returnvalue))
  ;[1 1 1] 上もしくは下にものがあるときは上下移動ボタンを押せなくする
  (if (== (Utilities|GetClass OtherActor) "/Game/Revive/Blueprints/Character/Copy_Blueprint.Copy_Blueprint_C")
    (if (Variables|/Game/Revive/Blueprints/Character/ThirdPersonCharacter.ThirdPersonCharacter_C|GetNot%20Up%20Down _asthird_person_character)
      (Variables|/Game/Revive/Blueprints/Character/ThirdPersonCharacter.ThirdPersonCharacter_C|SetNot%20Up%20Down _asthird_person_character false)
      (else
        (Variables|/Game/Revive/Blueprints/Character/ThirdPersonCharacter.ThirdPersonCharacter_C|SetNotUpDown2 _asthird_person_character false)))))

(event OnComponentBeginOverlap(Sphere)
  (params (OverlappedComponent :type Primitive%20Component%20Object%20Reference) (OtherActor :type Actor%20Object%20Reference) (OtherComp :type Primitive%20Component%20Object%20Reference) (OtherBodyIndex :type Integer) (bFromSweep :type Boolean) (SweepResult :type Hit%20Result%20Structure%20%28by%20ref%29))
  ;[1 1 1] プレイヤーとの当たり判定（放出・吸収用）
  (if (== (Utilities|GetClass OtherActor) "/Game/Revive/Blueprints/Character/ThirdPersonCharacter.ThirdPersonCharacter_C")
    (if (Components|ComponentHasTag OtherComp "PLAYER")
      (Class|HITBPIF|HitCall(Message) OtherActor true)
      (if (not (Variables|Default|GetPlayer_In))
        (Variables|Default|SetPlayer_In true)
        (if (>= (Variables|Default|GetP_HP) 1e+01)
          (Variables|Default|SetP_TIMEHP (Variables|Default|GetP_HP)))))))

(event OnComponentEndOverlap(Sphere)
  (params (OverlappedComponent :type Primitive%20Component%20Object%20Reference) (OtherActor :type Actor%20Object%20Reference) (OtherComp :type Primitive%20Component%20Object%20Reference) (OtherBodyIndex :type Integer))
  ;[1 1 1] プレイヤーとの当たり判定（放出・吸収用）
  (if (== (Utilities|GetClass OtherActor) "/Game/Revive/Blueprints/Character/ThirdPersonCharacter.ThirdPersonCharacter_C")
    (if (Components|ComponentHasTag OtherComp "PLAYER")
      (Class|HITBPIF|HitCall(Message) OtherActor false)
      (Variables|Default|SetPlayer_In false))))

(event OnComponentBeginOverlap(UP)
  (params (OverlappedComponent :type Primitive%20Component%20Object%20Reference) (OtherActor :type Actor%20Object%20Reference) (OtherComp :type Primitive%20Component%20Object%20Reference) (OtherBodyIndex :type Integer) (bFromSweep :type Boolean) (SweepResult :type Hit%20Result%20Structure%20%28by%20ref%29))
  (bind _returnvalue (Game|GetPlayerCharacter 0))
  (bind _asthird_person_character (Utilities|Casting|CastToThirdPersonCharacter _returnvalue))
  ;[1 1 1] 上もしくは下にものがあるときは上下移動ボタンを押せなくする
  (if (== (Utilities|GetClass OtherActor) "/Game/Revive/Blueprints/Character/Copy_Blueprint.Copy_Blueprint_C")
    (if (not (Variables|/Game/Revive/Blueprints/Character/ThirdPersonCharacter.ThirdPersonCharacter_C|GetNot%20Up%20Down _asthird_person_character))
      (Variables|/Game/Revive/Blueprints/Character/ThirdPersonCharacter.ThirdPersonCharacter_C|SetNot%20Up%20Down _asthird_person_character true))))

(event OnComponentBeginOverlap(DOWN)
  (params (OverlappedComponent :type Primitive%20Component%20Object%20Reference) (OtherActor :type Actor%20Object%20Reference) (OtherComp :type Primitive%20Component%20Object%20Reference) (OtherBodyIndex :type Integer) (bFromSweep :type Boolean) (SweepResult :type Hit%20Result%20Structure%20%28by%20ref%29))
  (bind _returnvalue (Game|GetPlayerCharacter 0))
  (bind _asthird_person_character (Utilities|Casting|CastToThirdPersonCharacter _returnvalue))
  ;[1 1 1] 上もしくは下にものがあるときは上下移動ボタンを押せなくする
  (if (== (Utilities|GetClass OtherActor) "/Game/Revive/Blueprints/Character/Copy_Blueprint.Copy_Blueprint_C")
    (if (Variables|/Game/Revive/Blueprints/Character/ThirdPersonCharacter.ThirdPersonCharacter_C|GetNot%20Up%20Down _asthird_person_character)
      (Variables|/Game/Revive/Blueprints/Character/ThirdPersonCharacter.ThirdPersonCharacter_C|SetNotUpDown2 _asthird_person_character true)
      (else
        (Variables|/Game/Revive/Blueprints/Character/ThirdPersonCharacter.ThirdPersonCharacter_C|SetNot%20Up%20Down _asthird_person_character true)))))

(event OnComponentEndOverlap(DOWN)
  (params (OverlappedComponent :type Primitive%20Component%20Object%20Reference) (OtherActor :type Actor%20Object%20Reference) (OtherComp :type Primitive%20Component%20Object%20Reference) (OtherBodyIndex :type Integer))
  (bind _returnvalue (Game|GetPlayerCharacter 0))
  (bind _asthird_person_character (Utilities|Casting|CastToThirdPersonCharacter _returnvalue))
  ;[1 1 1] 上もしくは下にものがあるときは上下移動ボタンを押せなくする
  (if (== (Utilities|GetClass OtherActor) "/Game/Revive/Blueprints/Character/Copy_Blueprint.Copy_Blueprint_C")
    (if (Variables|/Game/Revive/Blueprints/Character/ThirdPersonCharacter.ThirdPersonCharacter_C|GetNot%20Up%20Down _asthird_person_character)
      (Variables|/Game/Revive/Blueprints/Character/ThirdPersonCharacter.ThirdPersonCharacter_C|SetNot%20Up%20Down _asthird_person_character false)
      (else
        (Variables|/Game/Revive/Blueprints/Character/ThirdPersonCharacter.ThirdPersonCharacter_C|SetNotUpDown2 _asthird_person_character false)))))

(event Custom|CustomEvent
  (params (hitflag :type Boolean))
  ;[1 1 1] 上もしくは下にものがあるときは上下移動ボタンを押せなくする
  (Utilities|FlowControl|DoOnce false
    (:Completed
      (Actor|DestroyActor)
      (Variables|/Game/Revive/Blueprints/Character/ThirdPersonCharacter.ThirdPersonCharacter_C|SetNotUpDown2 (.AsThird%20Person%20Character (Utilities|Casting|CastToThirdPersonCharacter (Game|GetPlayerCharacter 0))) true))))

(event EventWakuseiHpAdd
  ;[1 1 1] HPを与える処理
  (if (Variables|Default|GetPlayer_In)
    (if (>= (Variables|Default|GetP_MAXHP) (Variables|Default|GetP_HP))
      (bind _output_get (Variables|Default|SetP_HP (+ (Variables|Default|GetP_HP) (Variables|Default|Gethp_add))))
      (Variables|Default|SetP_TIME_MAXHP _output_get))))

(event EventLineHit
  (params (flag :type Boolean))
  ;[1 1 1] BPIF取得
  (Variables|Default|Setplayer_hit flag))

(event EventSUIKOMIHIT
  (params (Flag :type Boolean))
  (Variables|Default|SetSUIKOMI Flag))

(event EventTick
  (params (DeltaSeconds :type Float%20%28single-precision%29))
  (bind _staticmeshcomponent (Variables|Debug|GetStaticMeshComponent))
  (bind _sphere1 (Variables|Default|GetSphere1))
  (bind _particlesystem1 (Variables|Default|GetParticleSystem1))
  (bind _p_hp (Variables|Default|GetP_HP))
  (bind _icegethp (Variables|Default|GetIceGetHp))
  (bind _particlesystem2 (Variables|Default|GetParticleSystem2))
  (bind _returnvalue (< 0.0 _icegethp))
  (bind _returnvalue_2 (* _p_hp 0.07))
  (bind _returnvalue_3 (Math|Float|Absolute(Float) _returnvalue_2))
  (Utilities|FlowControl|Sequence
    (:then_0
      ;[1 1 1] HPゲージが常にカメラを向くように設定
      (|CameraMove))
    (:then_1
      ;[1 1 1] HPの割合を求める
      (|HP＿WARIAI))
    (:then_2
      ;[1 1 1] パーティクルON/OFF
      (|Particle))
    (:then_3
      ;[1 1 1] 当たり判定の大きさ
      (if (> (Variables|Default|GetP_HP) 0.0)
        (bind _output_get (Variables|Default|Setscale_float _returnvalue_3))
        (if (>= _output_get 4.0)
          (Transformation|SetWorldScale3D _staticmeshcomponent "4.000000,4.000000,4.000000") ; 大きさが3以上だったら３にする
          (elif (>= 1.5 _output_get)
            (Transformation|SetWorldScale3D _staticmeshcomponent "1.500000,1.500000,1.500000") ; 大きさが3以上だったら３にする
            (Transformation|SetWorldScale3D _sphere1 "1.500000,1.500000,1.500000")
            (else
              (Transformation|SetWorldScale3D _staticmeshcomponent (Math|Conversions|ToVector(Float) _returnvalue_3)))))
        (Transformation|SetWorldScale3D (Variables|Default|GetSphere) (Variables|Default|GetLINHITSCALE))
        (Transformation|SetWorldScale3D _sphere1 "7.000000,8.000000,8.000000")
        (Transformation|SetWorldScale3D (Variables|Default|Getbakuha) (Variables|Default|GetBakuhaHanni))
        (Transformation|SetWorldScale3D (Variables|Default|GetEnergie) "2.500000,2.500000,2.500000")))
    (:then_4
      ;[1 1 1] 凍る見た目処理
      (if (Variables|Default|GetIceFlag)
        (if (not (Variables|Default|GetFireFlag))
          (Rendering|SetVisibility (Variables|Default|GetParticleSystem3) true false)
          (Components|Activation|Activate (Variables|Default|GetParticleSystem3) false) ; パーティクル再生
        )
        (else
          (Components|Activation|Deactivate (Variables|Default|GetParticleSystem3)) ; パーティクル停止
        )))
    (:then_5
      ;[1 1 1] パーティクル
      (if (<= (Variables|/Game/Revive/Blueprints/UI/Energie_UI.Energie_UI_C|GetEnergie (Variables|Default|GetEnergie_UI)) 0.3)
        (if (>= (Variables|/Game/Revive/Blueprints/UI/Energie_UI.Energie_UI_C|GetEnergie (Variables|Default|GetEnergie_UI)) 0.15)
          (Rendering|Material|SetMaterial (Variables|Debug|GetStaticMeshComponent) 0 "/Game/Revive/Models/Energy/EnergyMaterial.EnergyMaterial")
          (else
            (Rendering|Material|SetMaterial (Variables|Debug|GetStaticMeshComponent) 0 "/Game/Revive/Models/Energy/EnergyMaterial.EnergyMaterial")))
        (Transformation|SetWorldScale3D _particlesystem1 "2.000000,2.000000,2.000000")
        (Components|Activation|Activate _particlesystem1 false)
        (else
          (Components|Activation|Deactivate (Variables|Default|GetParticleSystem1)) ; パーティクル停止
        )))
    (:then_6
      ;[1 1 1] 星の回転
      (if (Math|Boolean|NotEqual(Boolean) (Variables|Default|GetPlayer_In) true) ; プレイヤーに接触してたら止まる
        (if (Variables|Default|GetZiku_In)
          (Transformation|AddActorLocalRotation (Variables|Default|GetRotationStarSpeed) false false)
          (bind _output_get_2 (Variables|Default|SetDirectionVector (Math|Rotator|GetRotationXVector (Transformation|GetActorRotation))))
          (Transformation|SetActorLocation (+ (Variables|Default|GetStartPosition) (* (Math|Vector|Normalize _output_get_2) (Variables|Default|GetDistance))) false false)
          (Development|PrintString (Utilities|String|ToString(Vector) (Variables|Default|GetRotationMove)) true true "(R=0.000000,G=0.660000,B=1.000000,A=1.000000)" 0.0))))
    (:then_7
      ;[1 1 1] 吸い込みUI
      (if (Variables|Default|Getplayer_hit)
        (if (Variables|Default|GetPlayer_In)
          (bind _asthird_person_character (Utilities|Casting|CastToThirdPersonCharacter (Game|GetPlayerCharacter 0)))
          (if (not (Variables|/Game/Revive/Blueprints/Character/ThirdPersonCharacter.ThirdPersonCharacter_C|GetChutoOn _asthird_person_character))
            (if (not (Variables|Default|GetIceFlag))
              (bind _returnvalue_4 (UserInterface|CreateWidget "/Game/Revive/Blueprints/UI/Suikomi_UI.Suikomi_UI_C"))
              (UserInterface|Viewport|AddtoViewport _returnvalue_4 0))))
        (else
          (bind _asthird_person_character_2 (Utilities|Casting|CastToThirdPersonCharacter (Game|GetPlayerCharacter 0)))
          (Variables|/Game/Revive/Blueprints/Character/ThirdPersonCharacter.ThirdPersonCharacter_C|Sethitflag _asthird_person_character_2 false))))
    (:then_8
      ;[1 1 1] 太陽で氷を溶かす処理
      (if (Variables|Default|GetFireFlag)
        (if (not (Variables|Default|GetIceFlag))
          (Utilities|FlowControl|DoOnce false :!label _label
            (:Completed
              (Rendering|SetVisibility (Variables|Default|GetParticleSystem2) true false)
              (Components|Activation|Activate (Variables|Default|GetParticleSystem2) false) ; パーティクル再生
              (Utilities|FlowControl|Delay 0.5)
              (Components|Activation|Deactivate _particlesystem2) ; パーティクル停止
            )))
        (else
          (Components|Activation|Deactivate _particlesystem2) ; パーティクル停止
          (goto _label Reset))))
    (:then_9
      (if true
        (if (< 0.0 (Variables|Default|GetFireGetHp))
          (if _returnvalue
            (if (<= (Variables|Default|GetIceGetHp) (Variables|Default|GetFireGetHp))
              (Variables|Default|SetFireFlag true :!label _label_2)
              (Variables|Default|SetIceFlag false)
              (else
                (Variables|Default|SetIceFlag true :!label _label_3)
                (Variables|Default|SetFireFlag false)))
            (else
              (goto _label_2)))
          (elif _returnvalue
            (goto _label_3)))))
    (:then_10
      (Transformation|SetWorldScale3D (Variables|Default|GetSphere) (Utilities|DEFINEWAKUSEILINEHITSCALE)))))

(event EventBeginPlay
  (bind _returnvalue (Transformation|GetActorLocation))
  ;[1 1 1] ウィジェット生成
  (bind _asenergie_ui (Utilities|Casting|CastToEnergie_UI (UserInterface|GetUserWidgetObject (Variables|Default|GetEnergie))))
  (bind _output_get (Variables|Default|SetEnergie_UI _asenergie_ui))
  (Variables|/Game/Revive/Blueprints/UI/Energie_UI.Energie_UI_C|SetEnergie _output_get 1.0)
  (bind _ashp_visible_ui (Utilities|Casting|CastToHP_Visible_UI (UserInterface|GetUserWidgetObject (Variables|Default|GetHP_Visibli))))
  (bind _output_get_2 (Variables|Default|SetHP_NUMBER _ashp_visible_ui))
  (Variables|/Game/Revive/Blueprints/UI/HP_Visible_UI.HP_Visible_UI_C|SetHP _output_get_2 (Variables|Default|GetP_MAXHP))
  (bind _output_get_3 (Variables|Default|SetP_HP (Variables|Default|GetP_MAXHP)))
  (Variables|Default|SetP_TIME_MAXHP _output_get_3)
  (Components|Activation|Deactivate (Variables|Default|GetParticleSystem)) ; パーティクル停止
  (Components|Activation|Deactivate (Variables|Default|GetParticleSystem1)) ; パーティクル停止
  (Variables|Default|SetStartPosition (Math|Vector|MakeVector (.x _returnvalue) (.y _returnvalue) (.z _returnvalue)))
  (Variables|Default|SetP_TIMEHP (Variables|Default|GetP_HP)))

(event EventHitCall
  (params (hitflag :type Boolean))
  ;[1 1 1] 上もしくは下にものがあるときは上下移動ボタンを押せなくする
  (Utilities|FlowControl|DoOnce false
    (:Completed
      (Actor|DestroyActor))))

(event EventZikuHanni
  (params (flag :type Boolean) (location :type Vector :default "0, 0, 0") (Component :type Static%20Mesh%20Component%20Object%20Reference))
  ;[1 1 1] 軸イベント
  (Variables|Default|SetZiku_In flag)
  (Variables|Default|SetRotationMove location))

(fn ConstructionScript
  (bind _returnvalue (Transformation|GetActorLocation))
  (bind _p_maxhp (Variables|Default|GetP_MAXHP))
  (bind _staticmeshcomponent (Variables|Debug|GetStaticMeshComponent))
  (bind _sphere1 (Variables|Default|GetSphere1))
  (bind _returnvalue_2 (* _p_maxhp 0.07))
  (bind _returnvalue_3 (Math|Float|Absolute(Float) _returnvalue_2))
  (Utilities|FlowControl|Sequence
    (:then_0
      (Rendering|SetVisibility (Variables|Default|GetSphere) (Variables|Default|Getsphere_look) false)
      (Rendering|SetVisibility (Variables|Default|GetSphere1) (Variables|Default|Getsphere1_look) false)
      (Rendering|SetVisibility (Variables|Default|Getbakuha) (Variables|Default|Getbakuha_look) false)
      (Rendering|SetVisibility (Variables|Default|GetUP) (Variables|Default|GetUP_look) false)
      (Rendering|SetVisibility (Variables|Default|GetDOWN) (Variables|Default|GetDOWN_look) false))
    (:then_1
      (Transformation|SetWorldScale3D (Variables|Default|Getbakuha) (Variables|Default|GetBakuhaHanni))
      (bind _output_get (Variables|Default|Setscale_float _returnvalue_3))
      (if (>= _output_get 4.0)
        (Transformation|SetWorldScale3D _staticmeshcomponent "4.000000,4.000000,4.000000") ; 大きさが3以上だったら３にする
        (elif (>= 1.5 _output_get)
          (Transformation|SetWorldScale3D _staticmeshcomponent "1.500000,1.500000,1.500000") ; 大きさが3以上だったら３にする
          (Transformation|SetWorldScale3D _sphere1 "1.500000,1.500000,1.500000")
          (else
            (Transformation|SetWorldScale3D _staticmeshcomponent (Math|Conversions|ToVector(Float) _returnvalue_3)))))
      (Transformation|SetWorldScale3D (Variables|Default|GetSphere) "10.000000,10.000000,10.000000")
      (Transformation|SetWorldScale3D _sphere1 "7.000000,8.000000,8.000000")
      (Rendering|SetVisibility (Variables|Default|GetSphere1) false false)
      (if (Variables|Default|GetUpdown_Judge)
        (Variables|Default|SetZ_Location 1.16e+03)
        (else
          (Variables|Default|SetZ_Location 2.3e+02)))
      (Transformation|SetActorLocation (Math|Vector|MakeVector (.x _returnvalue) (.y _returnvalue) (Variables|Default|GetZ_Location)) false false))
    (:then_2
      (Rendering|SetVisibility (Variables|Default|GetParticleSystem2) false false))))