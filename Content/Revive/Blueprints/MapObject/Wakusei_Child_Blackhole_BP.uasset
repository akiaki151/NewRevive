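; Planet child Blueprint that turns into a black hole paired with a white hole when its HP reaches zero.
; Overlapping the outer sphere starts pulling planets and the player in, and the inner warp collision sends them to the white hole.
; Tick drives all motion: distance-scaled pull and ejection for planets, and a shrink, hidden travel and regrow sequence for the player.
; Planets are signalled through interface messages.
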(event OnComponentEndOverlap(BlackHoleCollision)
  (params (OverlappedComponent :type Primitive%20Component%20Object%20Reference) (OtherActor :type Actor%20Object%20Reference) (OtherComp :type Primitive%20Component%20Object%20Reference) (OtherBodyIndex :type Integer))
  ;[1 1 1] BHとの当たり判定
  (if (Variables|Default|GetBHWHFlag)
    (if (== (Utilities|GetClass OtherActor) "/Game/Revive/Blueprints/Character/ThirdPersonCharacter.ThirdPersonCharacter_C")
      (if (Components|ComponentHasTag OtherComp "Player")
        (Variables|Default|SetBHPlayerSuikomiFlag false)))))

(event OnComponentBeginOverlap(BlackHoleCollision)
  (params (OverlappedComponent :type Primitive%20Component%20Object%20Reference) (OtherActor :type Actor%20Object%20Reference) (OtherComp :type Primitive%20Component%20Object%20Reference) (OtherBodyIndex :type Integer) (bFromSweep :type Boolean) (SweepResult :type Hit%20Result%20Structure%20%28by%20ref%29))
  ;[1 1 1] BHとの当たり判定
  (if (Variables|Default|GetBHWHFlag)
    (Utilities|FlowControl|Sequence
      (:then_0
        (bind _outactors (Actor|GetAllActorsOfClass "Wakusei_Child_Blackhole_BP_C"))
        (for _array_element _outactors
          (if (not (== _array_element OtherActor)) ; BHをはじく
            (if (Utilities|ClassIsChildOf (Utilities|GetClass OtherActor) "/Game/Revive/Blueprints/MapObject/Wakusei_Blueprint.Wakusei_Blueprint_C") ; 惑星かどうか
              (if (not (Variables|/Game/Revive/Blueprints/MapObject/Wakusei_Blueprint.Wakusei_Blueprint_C|GetWhiteHoleFlag _array_element))
                (if (not (Variables|/Game/Revive/Blueprints/MapObject/Wakusei_Blueprint.Wakusei_Blueprint_C|GetBlackHoleFlag _array_element))
                  (if (Components|ComponentHasTag OtherComp "sphere")
                    (bind _updowncheck (Class|BHBPIF2|BHBPIF2(Message) OtherActor (Transformation|GetWorldLocation (Variables|Default|GetStaticMeshComponent)) (Variables|Default|GetMyWhiteHole) (Variables|Default|GetUpdown_Judge)))
                    (if _updowncheck
                      (Audio|PlaySoundatLocation "/Game/Revive/Sound/SE/true/ブラックホール_吸い込み_Cue.ブラックホール_吸い込み_Cue" (Transformation|GetActorLocation) "0, 0, 0" 1.0 1.0 0.0 "/Game/Revive/Sound/SE/se_explosionAttenuation.se_explosionAttenuation" 0 0)))))))))
      (:then_1
        (if (== (Utilities|GetClass OtherActor) "/Game/Revive/Blueprints/Character/ThirdPersonCharacter.ThirdPersonCharacter_C") ; Playerかどうか
          (if (Components|ComponentHasTag OtherComp "Player")
            (Variables|Default|SetBHPlayerSuikomiFlag true)
            (Audio|PlaySoundatLocation "/Game/Revive/Sound/SE/true/ブラックホール_吸い込み_Cue.ブラックホール_吸い込み_Cue" (Transformation|GetActorLocation) "0, 0, 0" 1.0 1.0 0.0 "/Game/Revive/Sound/SE/se_explosionAttenuation.se_explosionAttenuation" 0 0)))))))

(event OnComponentBeginOverlap(WarpCollision)
  (params (OverlappedComponent :type Primitive%20Component%20Object%20Reference) (OtherActor :type Actor%20Object%20Reference) (OtherComp :type Primitive%20Component%20Object%20Reference) (OtherBodyIndex :type Integer) (bFromSweep :type Boolean) (SweepResult :type Hit%20Result%20Structure%20%28by%20ref%29))
  ;[1 1 1] ワープ処理
  (if (Variables|Default|GetBHWHFlag)
    (Utilities|FlowControl|Sequence
      (:then_0
        (if (not (Utilities|ClassIsChildOf (Utilities|GetClass OtherActor) "Wakusei_Child_Blackhole_BP_C")) ; BHをはじく
          (if (Utilities|ClassIsChildOf (Utilities|GetClass OtherActor) "/Game/Revive/Blueprints/MapObject/Wakusei_Blueprint.Wakusei_Blueprint_C") ; 惑星かどうか
            (if (Components|ComponentHasTag OtherComp "sphere")
              (Class|BHBPIF|BHBPIF(Message) OtherActor (Variables|Default|GetMyWhiteHole))
              (Audio|Components|Audio|Stop (Variables|Default|Getブラックホール引き寄せ))))))
      (:then_1
        (if (== (Utilities|GetClass OtherActor) "/Game/Revive/Blueprints/Character/ThirdPersonCharacter.ThirdPersonCharacter_C") ; Playerかどうか
          (if (Components|ComponentHasTag OtherComp "Player")
            (bind _asthird_person_character (Utilities|Casting|CastToThirdPersonCharacter (Game|GetPlayerCharacter 0)))
            (Variables|Default|SetBHPlayerSuikomiFlag false)
            (Variables|/Game/Revive/Blueprints/Character/ThirdPersonCharacter.ThirdPersonCharacter_C|SetWarpFlag _asthird_person_character true)
            (Variables|/Game/Revive/Blueprints/Character/ThirdPersonCharacter.ThirdPersonCharacter_C|SetScaleChange _asthird_person_character true)
            (Variables|Default|SetBHPlayerWarpFlag true)))))))

(event EventBeginPlay
  (|CallParentFunction)
  (Components|Sphere|SetSphereRadius (Variables|Default|GetBlackHoleCollision) (Variables|Default|GetBHRadius) true) ; 吸い込み範囲セット
  (Variables|Default|SetMyWhiteHole (Transformation|GetWorldLocation (Variables|Default|GetWhiteHole))) ; WHの位置セット
  (Transformation|SetWorldScale3D (Variables|Default|GetBlackHoleModel) "0, 0, 0")
  (Audio|Components|Audio|Stop (Variables|Default|Getブラックホール引き寄せ))
  (bind _asthird_person_character (Utilities|Casting|CastToThirdPersonCharacter (Game|GetPlayerCharacter 0)))
  (Variables|Default|SetKeepPlayerScale (Transformation|GetWorldScale (Variables|/Script/Engine.Character|GetMesh _asthird_person_character)))
  (Variables|Default|SetKeepPlayerLocation (Transformation|GetWorldLocation (Variables|/Script/Engine.Character|GetMesh _asthird_person_character)))
  (Transformation|SetWorldScale3D (Variables|Default|GetPlayerhit) "16.000000,16.000000,16.000000")
  (Components|Activation|Deactivate (Variables|Default|GetWHParticleSystem)) ; パーティクル停止
  (Variables|Default|SetP_HP 1e+01)
  (Variables|Default|SetP_MAXHP 1e+01))

(event Collision|EventActorBeginOverlap
  (params (OtherActor :type Actor%20Object%20Reference))
  (|CallParentFunction 0))

(event EventTick
  (params (DeltaSeconds :type Float%20%28single-precision%29))
  (bind _blackholecollision (Variables|Default|GetBlackHoleCollision))
  (bind _whparticlesystem (Variables|Default|GetWHParticleSystem))
  (bind _mywhitehole (Variables|Default|GetMyWhiteHole))
  (Transformation|SetWorldScale3D (Variables|Default|GetPlayerhit) (Utilities|DEFINEWAKUSEILINEHITSCALE))
  (Utilities|FlowControl|Sequence
    (:then_0
      (if (Variables|Default|GetBHWHFlag) ; BHが生成されているか
        (Utilities|FlowControl|Sequence
          (:then_0
            (bind _outactors (Actor|GetAllActorsOfClass "/Game/Revive/Blueprints/MapObject/Wakusei_Blueprint.Wakusei_Blueprint_C"))
            (for _array_element _outactors
              ;[1 1 1] BH吸い込み処理
              (if (Math|Vector|Equal(Vector) (Variables|/Game/Revive/Blueprints/MapObject/Wakusei_Blueprint.Wakusei_Blueprint_C|GetHWpos _array_element) (Variables|Default|GetMyWhiteHole) 0.0001)
                (Utilities|FlowControl|Sequence
                  (:then_0
                    (if (Variables|/Game/Revive/Blueprints/MapObject/Wakusei_Blueprint.Wakusei_Blueprint_C|GetBlackHoleFlag _array_element) ; BHに吸われているか
                      (Transformation|AddWorldOffset (Variables|/Script/Engine.StaticMeshActor|GetStaticMeshComponent _array_element) (* (Variables|/Game/Revive/Blueprints/MapObject/Wakusei_Blueprint.Wakusei_Blueprint_C|GetBHMove _array_element) (+ (Variables|Default|GetBHsuikomiSpeed) (* (/ (Math|Vector|VectorLength (- (Transformation|GetWorldLocation (Variables|Default|GetStaticMeshComponent)) (Transformation|GetWorldLocation (Variables|/Script/Engine.StaticMeshActor|GetStaticMeshComponent _array_element)))) (Variables|/Game/Revive/Blueprints/MapObject/Wakusei_Blueprint.Wakusei_Blueprint_C|GetLength _array_element)) 1e+01))) false false)))
                  (:then_1
                    (if (Variables|/Game/Revive/Blueprints/MapObject/Wakusei_Blueprint.Wakusei_Blueprint_C|GetWhiteHoleFlag _array_element) ; WHに吐き出されているか
                      ;;[1 1 1] WH吐き出し終了処理
                      (Transformation|AddActorWorldOffset _array_element (* (Variables|/Game/Revive/Blueprints/MapObject/Wakusei_Blueprint.Wakusei_Blueprint_C|GetBHMove _array_element) (+ (Variables|Default|GetBHsuikomiSpeed) (* (/ (Math|Vector|VectorLength (- (Transformation|GetWorldLocation (Variables|/Script/Engine.StaticMeshActor|GetStaticMeshComponent _array_element)) (Variables|Default|GetMyWhiteHole))) (Variables|Default|GetWHRadius)) 1e+01))))
                      (if (not (<= (Math|Vector|VectorLength (- (Transformation|GetWorldLocation (Variables|/Script/Engine.StaticMeshActor|GetStaticMeshComponent _array_element)) (Variables|Default|GetMyWhiteHole))) (Variables|Default|GetWHRadius))) ; WHの範囲に入っているか
                        (Variables|/Game/Revive/Blueprints/MapObject/Wakusei_Blueprint.Wakusei_Blueprint_C|SetWhiteHoleFlag _array_element false))))))))
          (:then_1
            ;[1 1 1] Player吸い込み処理
            (if (Variables|Default|GetBHPlayerSuikomiFlag)
              (bind _asthird_person_character (Utilities|Casting|CastToThirdPersonCharacter (Game|GetPlayerCharacter 0)))
              (Transformation|AddActorWorldOffset _asthird_person_character (* (Math|Vector|Normalize (- (Transformation|GetWorldLocation (Variables|Default|GetStaticMeshComponent)) (Transformation|GetWorldLocation (Variables|/Script/Engine.Actor|GetRootComponent _asthird_person_character)))) (* (Variables|Default|GetBHsuikomiSpeed) 6.0)))
              (Utilities|FlowControl|DoOnce false)))
          (:then_2
            ;[1 1 1] Playerワープ処理
            (if (Variables|Default|GetBHPlayerWarpFlag)
              (bind _asthird_person_character_2 (Utilities|Casting|CastToThirdPersonCharacter (Game|GetPlayerCharacter 0)))
              (if (Variables|/Game/Revive/Blueprints/Character/ThirdPersonCharacter.ThirdPersonCharacter_C|GetScaleChange _asthird_person_character_2)
                (if (Variables|Default|GetPlayerScaleReturn)
                  (Rendering|SetVisibility (Variables|/Script/Engine.Character|GetMesh _asthird_person_character_2) true false)
                  (Rendering|SetVisibility (Variables|/Script/Engine.Character|GetCapsuleComponent _asthird_person_character_2) true false)
                  (Collision|SetCollisionEnabled (Variables|/Script/Engine.Character|GetMesh _asthird_person_character_2) "QueryOnly")
                  (Transformation|SetWorldScale3D (Variables|/Script/Engine.Character|GetMesh _asthird_person_character_2) (/ (Transformation|GetWorldScale (Variables|/Script/Engine.Character|GetMesh _asthird_person_character_2)) 0.95))
                  (Transformation|AddWorldOffset (Variables|/Script/Engine.Character|GetMesh _asthird_person_character_2) "0, 0,-3.000000" false false)
                  (bind _result (Math|Integer|DecrementInt (Variables|Default|Getcount))
                    (:%20%20
                      (if (<= _result 0)
                        (Transformation|SetWorldScale3D (Variables|/Script/Engine.Character|GetMesh _asthird_person_character_2) (Variables|Default|GetKeepPlayerScale))
                        (Transformation|SetWorldLocation (Variables|/Script/Engine.Character|GetMesh _asthird_person_character_2) (Math|Vector|MakeVector (.x (Transformation|GetWorldLocation (Variables|/Script/Engine.Character|GetCapsuleComponent _asthird_person_character_2))) (.y (Transformation|GetWorldLocation (Variables|/Script/Engine.Character|GetCapsuleComponent _asthird_person_character_2))) (- (.z (Transformation|GetWorldLocation (Variables|/Script/Engine.Character|GetCapsuleComponent _asthird_person_character_2))) 97.0)) false false)
                        (Variables|Default|SetPlayerScaleReturn false)
                        (Variables|Default|SetBHPlayerWarpFlag false)
                        (Variables|/Game/Revive/Blueprints/Character/ThirdPersonCharacter.ThirdPersonCharacter_C|SetWarpFlag _asthird_person_character_2 false)
                        (Variables|/Game/Revive/Blueprints/Character/ThirdPersonCharacter.ThirdPersonCharacter_C|SetScaleChange _asthird_person_character_2 false)
                        (Variables|Default|SetBHPlayerSuikomiFlag false)
                        (Variables|Default|Setcount 0)
                        (goto _label Reset)
                        (else
                          (Utilities|FlowControl|DoOnce false :!label _label
                            (:Completed
                              (Audio|PlaySoundatLocation "/Game/Revive/Sound/SE/true/ブラックホール_出る_Cue.ブラックホール_出る_Cue" (Variables|Default|GetMyWhiteHole) "0, 0, 0" 2.0 1.0 0.0 "/Game/Revive/Sound/SE/se_explosionAttenuation.se_explosionAttenuation" 0 0)))))))
                  (else
                    (Transformation|SetWorldScale3D (Variables|/Script/Engine.Character|GetMesh _asthird_person_character_2) (* (Transformation|GetWorldScale (Variables|/Script/Engine.Character|GetMesh _asthird_person_character_2)) 0.95))
                    (Transformation|AddWorldOffset (Variables|/Script/Engine.Character|GetMesh _asthird_person_character_2) "0, 0,3.000000" false false)
                    (Math|Integer|IncrementInt (Variables|Default|Getcount)
                      (:%20%20
                        (if (>= (Variables|Default|Getcount) 30)
                          (Variables|/Game/Revive/Blueprints/Character/ThirdPersonCharacter.ThirdPersonCharacter_C|SetScaleChange _asthird_person_character_2 false))))))
                (elif (Variables|/Game/Revive/Blueprints/Character/ThirdPersonCharacter.ThirdPersonCharacter_C|GetWarpFlag _asthird_person_character_2)
                  (Transformation|AddActorWorldOffset _asthird_person_character_2 (* (Math|Vector|Normalize (- (Variables|Default|GetMyWhiteHole) (Transformation|GetWorldLocation (Variables|/Script/Engine.Actor|GetRootComponent _asthird_person_character_2)))) 1.2e+02) false true)
                  (Rendering|SetVisibility (Variables|/Script/Engine.Character|GetMesh _asthird_person_character_2) false false)
                  (Rendering|SetVisibility (Variables|/Script/Engine.Character|GetCapsuleComponent _asthird_person_character_2) false false)
                  (Collision|SetCollisionEnabled (Variables|/Script/Engine.Character|GetMesh _asthird_person_character_2) "NoCollision")
                  (if (<= (Math|Vector|VectorLength (- (Variables|Default|GetMyWhiteHole) (Transformation|GetWorldLocation (Variables|/Script/Engine.Actor|GetRootComponent _asthird_person_character_2)))) 6e+01)
                    (Variables|/Game/Revive/Blueprints/Character/ThirdPersonCharacter.ThirdPersonCharacter_C|SetScaleChange _asthird_person_character_2 true)
                    (Variables|Default|SetPlayerScaleReturn true))))))
          (:then_3
            ;[1 1 1] サイズ設定
            (Transformation|SetWorldScale3D (Variables|Default|GetBlackHoleModel) "1.000000,1.000000,1.000000") ; BHのパーティクル大きさ設定
            (Transformation|SetWorldScale3D (Variables|Default|GetSphere1) "0, 0, 0") ; 実体の当たり判定消去
            (Transformation|SetWorldScale3D _blackholecollision "1.000000,1.000000,1.000000") ; BHの大きさ固定(大きさ変える時はRadiusを変えて)
            (Transformation|SetWorldScale3D (Variables|Default|GetWarpCollision) "1.000000,1.000000,1.000000")
            (Transformation|SetWorldScale3D (Variables|Default|GetStaticMeshComponent) "0.010000,0.010000,0.010000")
            (Components|Sphere|SetSphereRadius _blackholecollision (Variables|Default|GetBHRadius) true))
          (:then_5
            (Development|PrintString (Utilities|String|ToString(Vector) (Variables|Default|GetHWpos)) true true "(R=0.643658,G=1.000000,B=0.000000,A=1.000000)" 0.0)))
        (else
          (|CallParentFunction DeltaSeconds)
          ;[1 1 1] HPが０になったらBH表示
          (if (<= (Variables|Default|GetP_HP) 0.0) ; HPが０になったらBH表示
            (Transformation|SetWorldScale3D (Variables|Default|GetStaticMeshComponent) "0.010000,0.010000,0.010000")
            (Transformation|SetWorldScale3D (Variables|Default|GetBlackHoleModel) "10.000000,10.000000,10.000000") ; BHの大きさ固定(大きさ変える時はRadiusを変えて)
            (Variables|Default|SetBHWHFlag true)
            (else
              (Transformation|SetWorldScale3D (Variables|Default|GetStaticMeshComponent) "1.000000,1.000000,1.000000")
              (Transformation|SetWorldScale3D (Variables|Default|GetSphere1) "4.000000,4.000000,4.000000"))))))
    (:then_1
      (if (Variables|Default|GetPlayer_In)
        (if (Variables|Default|Getplayer_hit)
          (Components|Activation|Activate _whparticlesystem false) ; パーティクル再生
          (Transformation|SetWorldLocation _whparticlesystem (Math|Vector|MakeVector (.x _mywhitehole) (.y _mywhitehole) (+ (.z _mywhitehole) 1e+02)) false false)
          (else
            (Components|Activation|Deactivate _whparticlesystem :!label _label_2) ; パーティクル停止
          ))
        (else
          (goto _label_2))))))

(fn ConstructionScript
  (|CallParentFunction)
  (Components|Sphere|SetSphereRadius (Variables|Default|GetBlackHoleCollision) (Variables|Default|GetBHRadius) true))

(fn BHWakuseiBPIF
  (params (LOCATION :type Vector :default "0, 0, 0") (HWpos :type Vector :default "0, 0, 0") (UpDownFlag :type Boolean))
  (return))