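; Wakusei_Infinite_BP is an exploding planet map object that respawns endlessly.
; Its HP drains while the player's MoveFlag is set, barring ice or held inputs, and any damage zeroes it; low HP changes material and particles.
; At zero it explodes, damaging the player and other planet types or hitting break walls through blast-sphere overlaps.
; Before expiring, it spawns its replacement with saved initial stats and a height-based up/down flag.
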(event OnComponentEndOverlap(bakuha)
  (params (OverlappedComponent :type Primitive%20Component%20Object%20Reference) (OtherActor :type Actor%20Object%20Reference) (OtherComp :type Primitive%20Component%20Object%20Reference) (OtherBodyIndex :type Integer))
  ;[1 1 1] 爆破したら範囲内のプレイヤーと惑星を爆破する
  (if (Variables|Default|Getdeath)
    (if (== (Utilities|GetClass OtherActor) "/Game/Revive/Blueprints/Character/ThirdPersonCharacter.ThirdPersonCharacter_C")
      (Utilities|FlowControl|DoOnce false
        (:Completed
          (Class|WakuseiLocationBPIF|WakuseiLocation(Message) OtherActor (Transformation|GetWorldLocation (Variables|Default|GetStaticMeshComponent)))
          (Game|Damage|ApplyDamage OtherActor (Variables|Default|GetDamage) 0 0)))
      (elif (== (Utilities|GetClass OtherActor) "/Game/Revive/Blueprints/MapObject/BreakWall_BP1.BreakWall_BP1_C")
        (Class|HITBPIF|HitCall(Message) OtherActor false)
        (elif (Class|PrimitiveComponent|IsOverlappingComponent (Variables|Default|GetSphere) OtherComp)
          (if (!= (Utilities|GetClass OtherActor) "Wakusei_Infinite_BP_C")
            (Game|Damage|ApplyDamage OtherActor 1.0 0 0)))))))

(event OnComponentBeginOverlap(bakuha)
  (params (OverlappedComponent :type Primitive%20Component%20Object%20Reference) (OtherActor :type Actor%20Object%20Reference) (OtherComp :type Primitive%20Component%20Object%20Reference) (OtherBodyIndex :type Integer) (bFromSweep :type Boolean) (SweepResult :type Hit%20Result%20Structure%20%28by%20ref%29))
  ;[1 1 1] 爆破したら範囲内のプレイヤーと惑星を爆破する
  (if (Variables|Default|Getdeath)
    (if (Class|PrimitiveComponent|IsOverlappingComponent (Variables|Default|GetSphere) OtherComp)
      (if (!= (Utilities|GetClass OtherActor) "Wakusei_Infinite_BP_C")
        (Game|Damage|ApplyDamage OtherActor 1.0 0 0)))))

(event EventBeginPlay
  (bind _p_hp (Variables|Default|GetP_HP))
  (|CallParentFunction)
  (Variables|Default|SetP_MAXHP _p_hp)
  (bind _output_get (Variables|Default|SetP_TIME_MAXHP _p_hp))
  (Variables|Default|SetP_TIMEHP _output_get)
  (Variables|Default|SetInfiniteHP _p_hp)
  (Variables|Default|SetInfiniteDamage (Variables|Default|GetDamage))
  (Variables|Default|SetInfiniteDistance (Variables|Default|GetDistance))
  (Variables|Default|SetInfiniteBakuha (Variables|Default|GetBakuhaHanni))
  (if (< 0.0 (.z (Variables|Default|Getstart%20location)))
    (Variables|Default|SetStartPosition (Variables|Default|Getstart%20location))
    (else
      (Variables|Default|Setstart%20location (Variables|Default|GetStartPosition)))))

(event Collision|EventActorBeginOverlap
  (params (OtherActor :type Actor%20Object%20Reference))
  (|CallParentFunction OtherActor) ; This node is disabled and will not be called.\nDrag off pins to build functionality.
)

(event Game|Damage|EventAnyDamage
  (params (Damage :type Float%20%28single-precision%29) (DamageType :type Damage%20Type%20Object%20Reference) (InstigatedBy :type Controller%20Object%20Reference) (DamageCauser :type Actor%20Object%20Reference))
  (bind _returnvalue (Game|GetPlayerController 0))
  ;[1 1 1] 他の惑星の爆発に巻き込まれたら少し待って爆破する
  (Utilities|FlowControl|Delay 0.02)
  (Variables|Default|SetP_HP 0.0)
  (Variables|Default|SetP_TIME_MAXHP (Variables|Default|GetP_HP))
  (Class|PlayerCameraManager|PlayCameraShake (Variables|/Script/Engine.PlayerController|GetPlayerCameraManager _returnvalue) "/Game/Revive/Blueprints/MyCameraShake.MyCameraShake_C" 1.0 "CameraLocal" "0, 0, 0")
  (Game|Feedback|ClientPlayForceFeedback _returnvalue "/Game/Revive/Blueprints/NewForceFeedbackEffect.NewForceFeedbackEffect" "None" false false false))

(event EventTick
  (params (DeltaSeconds :type Float%20%28single-precision%29))
  (bind _returnvalue (Game|GetPlayerController 0))
  (bind _bakuha_collision (Variables|Default|Getbakuha_collision))
  (bind _particlesystem1 (Variables|Default|GetParticleSystem1))
  (bind _bakuhahanni (Variables|Default|GetBakuhaHanni))
  (bind _start_location (Variables|Default|Getstart%20location))
  (bind _infinitehp (Variables|Default|GetInfiniteHP))
  (|CallParentFunction DeltaSeconds)
  (Utilities|FlowControl|Sequence
    (:then_0
      ;[1 1 1] HPが0以下になったら爆発する
      (if (<= (Variables|Default|GetP_HP) 0.0)
        (Utilities|FlowControl|Sequence
          (:then_0
            (Utilities|FlowControl|DoOnce false
              (:Completed
                (Audio|PlaySoundatLocation "/Game/Revive/Sound/SE/true/爆発_re_Cue.爆発_re_Cue" (Transformation|GetActorLocation) "0, 0, 0" 1.0 1.0 0.0 "/Game/Revive/Sound/SE/se_explosionAttenuation.se_explosionAttenuation" 0 0)
                (Effects|SpawnEmitteratLocation "/Game/Revive/Effects/explosion.explosion" (Transformation|GetWorldLocation (Variables|Default|GetStaticMeshComponent)) "0, 0, 0" (* (Variables|Default|GetBakuhaHanni) 0.1))
                (Variables|Default|Setdeath true)
                (Actor|SetLifeSpan 0.02)
                (Class|PlayerCameraManager|PlayCameraShake (Variables|/Script/Engine.PlayerController|GetPlayerCameraManager _returnvalue) "/Game/Revive/Blueprints/MyCameraShake.MyCameraShake_C" 1.0 "CameraLocal" "0, 0, 0") ; カメラ振動
                (Game|Feedback|ClientPlayForceFeedback _returnvalue "/Game/Revive/Blueprints/NewForceFeedbackEffect.NewForceFeedbackEffect" "None" false false false)
                (if (<= (.z (Transformation|GetWorldLocation (Variables|Default|GetStaticMeshComponent))) 5e+02)
                  (Variables|Default|SetInfiniteUpDown false)
                  (else
                    (Variables|Default|SetInfiniteUpDown true))))))
          (:then_1
            (bind _result (Math|Float|IncrementFloat (Variables|Default|GetRespawn))
              (:%20%20
                (Development|PrintString (Utilities|String|ToString(Float) _result))))))))
    (:then_1
      ;[1 1 1] マテリアル変更
      (if (<= (Variables|/Game/Revive/Blueprints/UI/HP_UI.HP_UI_C|GetHP (Variables|Default|GetHP_UI)) 0.3)
        (if (>= (Variables|/Game/Revive/Blueprints/UI/HP_UI.HP_UI_C|GetHP (Variables|Default|GetHP_UI)) 0.15)
          (Rendering|Material|SetMaterial (Variables|Default|GetStaticMeshComponent) 0 "/DatasmithContent/Materials/CE_OpaqueMaster.CE_OpaqueMaster")
          (else
            (Rendering|Material|SetMaterial (Variables|Default|GetStaticMeshComponent) 0 "/DatasmithContent/Materials/FBXImporter/DeltaGenMasterTransparent.DeltaGenMasterTransparent")))
        (Transformation|SetWorldScale3D _particlesystem1 "2.000000,2.000000,2.000000")
        (Components|Activation|Activate _particlesystem1 false)
        (else
          (Components|Activation|Deactivate (Variables|Default|GetParticleSystem1)) ; パーティクル停止
        )))
    (:then_2
      ;[1 1 1] 星の復活
      (if (<= 2.0 (Variables|Default|GetRespawn))
        (Utilities|FlowControl|DoOnce false
          (:Completed
            (Game|SpawnActorfromClass "Wakusei_Infinite_BP_C" (Transformation|GetWorldTransform (Variables|Default|GetStaticMeshComponent)) "Undefined" 0 _start_location _infinitehp _infinitehp (Variables|Default|GetInfiniteBakuha) _start_location (Variables|Default|GetInfiniteDistance) (Variables|Default|GetInfiniteDamage) (Variables|Default|GetInfiniteUpDown) 0)))))
    (:then_3
      (bind _asthird_person_character (Utilities|Casting|CastToThirdPersonCharacter (Game|GetPlayerCharacter 0)))
      (if (Variables|/Game/Revive/Blueprints/Character/ThirdPersonCharacter.ThirdPersonCharacter_C|GetMoveFlag _asthird_person_character)
        (if (not (Variables|Default|GetIceFlag))
          (if (not (Variables|/Game/Revive/Blueprints/Character/ThirdPersonCharacter.ThirdPersonCharacter_C|Getspace_hold _asthird_person_character))
            (if (not (Variables|/Game/Revive/Blueprints/Character/ThirdPersonCharacter.ThirdPersonCharacter_C|Getenter_hold _asthird_person_character))
              (Variables|Default|SetP_HP (- (Variables|Default|GetP_HP) 0.1)))))))
    (:then_4
      (Transformation|SetWorldScale3D (Variables|Default|GetStaticMeshComponent) "4.000000,4.000000,4.000000") ; 大きさが3以上だったら３にする
      (Transformation|SetWorldScale3D (Variables|Default|GetSphere1) "4.000000,4.000000,4.000000")
      (Transformation|SetWorldScale3D (Variables|Default|GetSphere) "10.000000,10.000000,10.000000")
      (Transformation|SetWorldScale3D (Variables|Default|GetHP) "2.500000,2.500000,2.500000")
      (Transformation|SetWorldScale3D (Variables|Default|GetPlayerhit) (Utilities|DEFINEWAKUSEILINEHITSCALE))
      (Transformation|SetWorldScale3D (Variables|Default|GetAction_Collision) "4.000000,4.000000,4.000000")
      (Transformation|SetWorldScale3D _bakuha_collision (Math|Vector|MakeVector (* (/ (.x _bakuhahanni) 5.0) 3.0) (* (/ (.y _bakuhahanni) 5.0) 3.0) 0.01))
      (Transformation|SetWorldLocation _bakuha_collision (Math|Vector|MakeVector (.x (Variables|Default|GetInifinitestartposition)) (.y (Variables|Default|GetInifinitestartposition)) (- (.z (Variables|Default|GetInifinitestartposition)) 2.3e+02)) false false))
    (:then_5
      (Variables|Default|SetInifinitestartposition (Transformation|GetActorLocation))
      (Variables|Default|SetRotationStop false))
    (:then_6
      (Development|PrintString (Utilities|String|ToString(Vector) (Variables|Default|Getstart%20location)) true true "(R=0.000000,G=1.000000,B=0.322387,A=1.000000)" 0.0))
    (:then_7
      (Transformation|SetWorldScale3D (Variables|Default|Getbakuha) (Variables|Default|GetBakuhaHanni)))
    (:then_8
      (Development|PrintString (Utilities|String|ToString(Float) (Variables|Default|GetInfiniteDistance)) true true "(R=0.000000,G=1.000000,B=0.322387,A=1.000000)" 0.0))
    (:then_9
      (Development|PrintString (Utilities|String|ToString(Boolean) (Variables|Default|GetZiku_In)) true true "(R=0.000000,G=1.000000,B=0.316208,A=1.000000)" 0.0))
    (:then_10
      (Development|PrintString (Utilities|String|ToString(Boolean) (Variables|Default|GetRotationStop)) true true "(R=0.000000,G=1.000000,B=0.322387,A=1.000000)" 0.0))))

(fn ConstructionScript
  (|CallParentFunction))