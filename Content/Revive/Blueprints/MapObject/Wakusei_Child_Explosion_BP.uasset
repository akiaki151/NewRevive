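; Explosive child planet (Wakusei) whose HP drains while the player's move flag is set, unless iced or Space/Enter is held.
; Tick blinks its material at low HP, resolves fire/ice state and shows a blast-range marker matching the player's up/down side.
; At zero HP it explodes with effects and a short lifespan.
; Blast-sphere end-overlaps after death damage players, break walls and chain-detonate other explosive planets after a delay.
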(event OnComponentEndOverlap(bakuha)
  (params (OverlappedComponent :type Primitive%20Component%20Object%20Reference) (OtherActor :type Actor%20Object%20Reference) (OtherComp :type Primitive%20Component%20Object%20Reference) (OtherBodyIndex :type Integer))
  ;[1 1 1] 爆破したら範囲内のプレイヤーと惑星を爆破する
  (if (Variables|Default|Getdeath)
    (Utilities|FlowControl|Sequence
      (:then_0
        (if (== (Utilities|GetClass OtherActor) "/Game/Revive/Blueprints/Character/ThirdPersonCharacter.ThirdPersonCharacter_C")
          (Utilities|FlowControl|DoOnce false
            (:Completed
              (Class|WakuseiLocationBPIF|WakuseiLocation(Message) OtherActor (Transformation|GetWorldLocation (Variables|Default|GetStaticMeshComponent)))
              (Game|Damage|ApplyDamage OtherActor (Variables|Default|GetDamage) 0 0)))))
      (:then_1
        (if (== (Utilities|GetClass OtherActor) "Wakusei_Child_Explosion_BP_C")
          (if (Components|ComponentHasTag OtherComp "aiba")
            (Class|HITBPIF|HitCall(Message) OtherActor false))))
      (:then_2
        (if (== (Utilities|GetClass OtherActor) "/Game/Revive/Blueprints/MapObject/BreakWall_BP.BreakWall_BP_C")
          (Utilities|IsValid OtherActor
            (:Is%20Valid
              (Class|HITBPIF|HitCall(Message) OtherActor false))))))))

(event OnComponentBeginOverlap(bakuha)
  (params (OverlappedComponent :type Primitive%20Component%20Object%20Reference) (OtherActor :type Actor%20Object%20Reference) (OtherComp :type Primitive%20Component%20Object%20Reference) (OtherBodyIndex :type Integer) (bFromSweep :type Boolean) (SweepResult :type Hit%20Result%20Structure%20%28by%20ref%29))
  ;[1 1 1] 爆破したら範囲内のプレイヤーと惑星を爆破する
)

(event Custom|HitBakuha
  (bind _returnvalue (Game|GetPlayerController 0))
  ;[1 1 1] 他の惑星の爆発に巻き込まれたら少し待って爆破する
  (Utilities|FlowControl|Delay 0.2)
  (Variables|Default|SetP_HP 0.0)
  (Variables|Default|SetP_TIME_MAXHP (Variables|Default|GetP_HP))
  (Class|PlayerCameraManager|PlayCameraShake (Variables|/Script/Engine.PlayerController|GetPlayerCameraManager _returnvalue) "/Game/Revive/Blueprints/MyCameraShake.MyCameraShake_C" 1.0 "CameraLocal" "0, 0, 0")
  (Game|Feedback|ClientPlayForceFeedback _returnvalue "/Game/Revive/Blueprints/NewForceFeedbackEffect.NewForceFeedbackEffect" "None" false false false))

(event Collision|EventActorBeginOverlap
  (params (OtherActor :type Actor%20Object%20Reference))
  (|CallParentFunction OtherActor)
  (Transformation|SetWorldScale3D (Variables|Default|Getbakuha) (Variables|Default|GetBakuhaHanni)))

(event Game|Damage|EventAnyDamage
  (params (Damage :type Float%20%28single-precision%29) (DamageType :type Damage%20Type%20Object%20Reference) (InstigatedBy :type Controller%20Object%20Reference) (DamageCauser :type Actor%20Object%20Reference))
  (bind _returnvalue (Game|GetPlayerController 0))
  ;[1 1 1] 他の惑星の爆発に巻き込まれたら少し待って爆破する
  (Utilities|FlowControl|Delay 0.2)
  (Variables|Default|SetP_HP 0.0)
  (Variables|Default|SetP_TIME_MAXHP (Variables|Default|GetP_HP))
  (Class|PlayerCameraManager|PlayCameraShake (Variables|/Script/Engine.PlayerController|GetPlayerCameraManager _returnvalue) "/Game/Revive/Blueprints/MyCameraShake.MyCameraShake_C" 1.0 "CameraLocal" "0, 0, 0")
  (Game|Feedback|ClientPlayForceFeedback _returnvalue "/Game/Revive/Blueprints/NewForceFeedbackEffect.NewForceFeedbackEffect" "None" false false false))

(event EventTick
  (params (DeltaSeconds :type Float%20%28single-precision%29))
  (bind _returnvalue (Game|GetPlayerController 0))
  (bind _bakuha_collision (Variables|Default|Getbakuha_collision))
  (bind _particlesystem1 (Variables|Default|GetParticleSystem1))
  (bind _bakuhahanni (Variables|Default|GetBakuhaHanni))
  (bind _staticmeshcomponent (Variables|Default|GetStaticMeshComponent))
  (bind _bakuha_collision_2 (Variables|Default|Getbakuha_collision))
  (|CallParentFunction DeltaSeconds)
  (Utilities|FlowControl|Sequence
    (:then_0
      ;[1 1 1] HPが0以下になったら爆発する
      (if (<= (Variables|Default|GetP_HP) 0.0)
        (Utilities|FlowControl|DoOnce false
          (:Completed
            (Audio|PlaySoundatLocation "/Game/Revive/Sound/SE/true/爆発_re_Cue.爆発_re_Cue" (Transformation|GetActorLocation) "0, 0, 0" 1.0 1.0 0.0 "/Game/Revive/Sound/SE/se_explosionAttenuation.se_explosionAttenuation" 0 0)
            (Effects|SpawnEmitteratLocation "/Game/Revive/Effects/explosion.explosion" (Transformation|GetWorldLocation (Variables|Default|GetStaticMeshComponent)) "0, 0, 0" (* (Variables|Default|GetBakuhaHanni) 0.1))
            (Variables|Default|Setdeath true)
            (Actor|SetLifeSpan 0.2)
            (Class|PlayerCameraManager|PlayCameraShake (Variables|/Script/Engine.PlayerController|GetPlayerCameraManager _returnvalue) "/Game/Revive/Blueprints/MyCameraShake.MyCameraShake_C" 2.0 "CameraLocal" "0, 0, 0") ; カメラ振動
            (Game|Feedback|ClientPlayForceFeedback _returnvalue "/Game/Revive/Blueprints/NewForceFeedbackEffect.NewForceFeedbackEffect" "None" false false false)))))
    (:then_1
      ;[1 1 1] マテリアル変更
      (if (<= (Variables|/Game/Revive/Blueprints/UI/HP_UI.HP_UI_C|GetHP (Variables|Default|GetHP_UI)) 0.3)
        (if (>= (Variables|/Game/Revive/Blueprints/UI/HP_UI.HP_UI_C|GetHP (Variables|Default|GetHP_UI)) 0.15)
          (Rendering|Material|SetMaterial (Variables|Default|GetStaticMeshComponent) 0 "/Game/NormalWakusei/lambert3.lambert3")
          (elif (<= 15 (Variables|Default|Getcount))
            (Rendering|Material|SetMaterial _staticmeshcomponent 0 "/Game/NormalWakusei/lambert2.lambert2")
            (else
              (Rendering|Material|SetMaterial _staticmeshcomponent 0 "/Game/NormalWakusei/lambert1.lambert1"))))
        (Transformation|SetWorldScale3D _particlesystem1 "2.000000,2.000000,2.000000")
        (Components|Activation|Activate _particlesystem1 false)
        (else
          (Components|Activation|Deactivate (Variables|Default|GetParticleSystem1)) ; パーティクル停止
          (Rendering|Material|SetMaterial _staticmeshcomponent 0 "/Game/NormalWakusei/lambert1.lambert1"))))
    (:then_2
      (Variables|Default|Setcount (+ (Variables|Default|Getcount) 1))
      (if (<= 30 (Variables|Default|Getcount))
        (Variables|Default|Setcount 0)))
    (:then_3
      (bind _asthird_person_character (Utilities|Casting|CastToThirdPersonCharacter (Game|GetPlayerCharacter 0)))
      (if (Variables|/Game/Revive/Blueprints/Character/ThirdPersonCharacter.ThirdPersonCharacter_C|GetMoveFlag _asthird_person_character)
        (if (not (Variables|Default|GetIceFlag))
          (if (not (Variables|/Game/Revive/Blueprints/Character/ThirdPersonCharacter.ThirdPersonCharacter_C|Getspace_hold _asthird_person_character))
            (if (not (Variables|/Game/Revive/Blueprints/Character/ThirdPersonCharacter.ThirdPersonCharacter_C|Getenter_hold _asthird_person_character))
              (Variables|Default|SetP_HP (- (Variables|Default|GetP_HP) 0.1)))))))
    (:then_4
      (Transformation|SetWorldScale3D _bakuha_collision (Math|Vector|MakeVector (* (/ (.x _bakuhahanni) 5.0) 3.0) (* (/ (.y _bakuhahanni) 5.0) 3.0) 0.01))
      (Transformation|SetWorldLocation _bakuha_collision (Math|Vector|MakeVector (.x (Variables|Default|Getbakuha_location)) (.y (Variables|Default|Getbakuha_location)) (- (.z (Variables|Default|Getbakuha_location)) 2.3e+02)) false false))
    (:then_5
      (Variables|Default|Setbakuha_location (Transformation|GetActorLocation)))
    (:then_6
      (bind _outactors (Actor|GetAllActorsOfClass "/Game/Revive/Blueprints/Character/ThirdPersonCharacter.ThirdPersonCharacter_C"))
      (for _array_element _outactors
        (if (Math|Boolean|Equal(Boolean) (Variables|Default|GetUpdown_Judge) (Variables|/Game/Revive/Blueprints/Character/ThirdPersonCharacter.ThirdPersonCharacter_C|GetPlayerUP _array_element))
          (Rendering|SetVisibility _bakuha_collision_2 true false)
          (else
            (Rendering|SetVisibility _bakuha_collision_2 false false)))))
    (:then_7
      (Transformation|SetWorldScale3D (Variables|Default|GetPlayerhit) (Utilities|DEFINEWAKUSEILINEHITSCALE)))
    (:then_8
      (if (< 0.0 (Variables|Default|GetFireGetHp))
        (if (< 0.0 (Variables|Default|GetIceGetHp))
          (if (<= (Variables|Default|GetIceGetHp) (Variables|Default|GetFireGetHp))
            _
            (else
              (Variables|Default|SetIceFlag true :!label _label)
              (Variables|Default|SetFireFlag false)
              (Utilities|FlowControl|DoOnce false :!label _label_2
                (:Completed
                  (Audio|PlaySoundatLocation "/Game/Revive/Sound/SE/true/凍らせる_re_Cue.凍らせる_re_Cue" (Transformation|GetActorLocation) "0, 0, 0" 1.0 1.0 0.0 "/Game/Revive/Sound/SE/se_explosionAttenuation.se_explosionAttenuation" 0 0)
                  (goto _label_3 Reset))))))
        (Variables|Default|SetFireFlag true)
        (Variables|Default|SetIceFlag false)
        (Utilities|FlowControl|DoOnce false :!label _label_3
          (:Completed
            (Audio|PlaySoundatLocation "/Game/Revive/Sound/SE/true/溶ける__re_Cue.溶ける__re_Cue" (Transformation|GetActorLocation) "0, 0, 0" 1.0 1.0 0.0 "/Game/Revive/Sound/SE/se_explosionAttenuation.se_explosionAttenuation" 0 0)
            (goto _label_2 Reset)))
        (elif (< 0.0 (Variables|Default|GetIceGetHp))
          (goto _label))))))

(event EventHitCall
  (params (hitflag :type Boolean))
  (bind _returnvalue (Game|GetPlayerController 0))
  ;[1 1 1] 他の惑星の爆発に巻き込まれたら少し待って爆破する
  (Utilities|FlowControl|Delay 0.2)
  (Variables|Default|SetP_HP 0.0)
  (Variables|Default|SetP_TIME_MAXHP (Variables|Default|GetP_HP))
  (Class|PlayerCameraManager|PlayCameraShake (Variables|/Script/Engine.PlayerController|GetPlayerCameraManager _returnvalue) "/Game/Revive/Blueprints/MyCameraShake.MyCameraShake_C" 1.0 "CameraLocal" "0, 0, 0")
  (Game|Feedback|ClientPlayForceFeedback _returnvalue "/Game/Revive/Blueprints/NewForceFeedbackEffect.NewForceFeedbackEffect" "None" false false false))

(fn ConstructionScript
  (|CallParentFunction))