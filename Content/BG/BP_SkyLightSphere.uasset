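; BP_SkyLightSphere is an environment actor that combines a textured sky sphere, an optional sky light and a configurable sun.
; Its Construction Script feeds one sky texture to both the SkyLight cubemap and a dynamic material on the sphere.
; A mobility enum shows one of three pre-placed static, stationary or movable suns, or none.
; The active sun receives rotation, color and intensity, and its pitch and yaw also yield a distant virtual sun position.
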(fn ConstructionScript
  (bind _skylight (Variables|Default|GetSkyLight))
  (bind _sunyaw (Variables|Default|GetSunYaw))
  (bind _skytexture (Variables|Default|GetSkyTexture))
  (bind _sunpitch (Variables|Default|GetSunPitch))
  (bind _skysphere (Variables|Default|GetSkySphere))
  (bind _returnvalue (* _sunpitch -1.0))
  (bind _returnvalue_2 (+ _sunyaw 9e+01))
  (bind _returnvalue_3 (Math|Rotator|MakeRotator 0.0 _returnvalue _returnvalue_2))
  (Rendering|SetVisibility _skylight (Variables|Default|GetUseItAsSkyLight) false)
  (Rendering|Components|Light|SetIntensity _skylight (Variables|Default|GetSkyIntensity))
  (Class|SkyLightComponent|SetCubemap _skylight _skytexture)
  (bind _returnvalue_4 (Rendering|Material|CreateDynamicMaterialInstance _skysphere 0 (Rendering|Material|GetMaterial _skysphere 0) "None" :!class /Script/Engine.PrimitiveComponent))
  (Rendering|Material|SetTextureParameterValue _returnvalue_4 "SkyTexture" _skytexture)
  (Rendering|Material|SetMaterial _skysphere 0 _returnvalue_4)
  (switch Utilities|FlowControl|Switch|Switchon (Variables|Default|GetSunMobilityType)
    (:NewEnumerator1
      (Rendering|SetVisibility false false)
      (Rendering|SetVisibility false false)
      (Rendering|SetVisibility false false))
    (:NewEnumerator4
      (Rendering|SetVisibility true false)
      (Rendering|SetVisibility false false)
      (Rendering|SetVisibility false false)
      (LocalVariables|SetActiveSun (Variables|Default|GetStaticSun))
      (Variables|Default|SetVirtualSunPosition (Math|Vector|RotateVector "-100000000.000000,0.000000, 0" _returnvalue_3) :!label _label)
      (Transformation|SetRelativeRotation (LocalVariables|GetActiveSun) _returnvalue_3 false false)
      (Rendering|Components|Light|SetLightColor (LocalVariables|GetActiveSun) (Variables|Default|GetSunColor) true)
      (Rendering|Components|Light|SetIntensity (LocalVariables|GetActiveSun) (Variables|Default|GetSunIntensity)))
    (:NewEnumerator2
      (Rendering|SetVisibility false false)
      (Rendering|SetVisibility true false)
      (Rendering|SetVisibility false false)
      (LocalVariables|SetActiveSun (Variables|Default|GetStationarySun))
      (goto _label))
    (:NewEnumerator3
      (Rendering|SetVisibility false false)
      (Rendering|SetVisibility false false)
      (Rendering|SetVisibility true false)
      (LocalVariables|SetActiveSun (Variables|Default|GetMovableSun))
      (goto _label))))